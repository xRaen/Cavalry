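; BP_CavalryPlayerCharacter is a VR player character with stick-driven movement and snap turning.
; The left stick moves along the actor's forward and right vectors, while the right stick yaws by a fixed angle once per push past a threshold.
; BeginPlay caches the camera's relative height and spawns left and right BP_MotionController actors attached to the capsule.
; Tick sets the capsule half-height to that cached height, not the live camera position.
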(event `InputAxis|LeftVerticalAxis`
  (params (AxisValue :type "Float (single-precision)"))
  ;[0 0 0] Controller based movement
  ;;[0.25 0.25 0.25] Moves the character forward/backward
  (`self.AddMovementInput` (`self.GetActorForwardVector`) AxisValue))

(event `InputAxis|LeftHorizontalAxis`
  (params (AxisValue :type "Float (single-precision)"))
  ;[0 0 0] Controller based movement
  ;;[0.25 0.25 0.25] Moves the character left/right
  (`self.AddMovementInput` (`self.GetActorRightVector`) AxisValue))

(event `InputAxis|RightHorizontalAxis`
  (params (AxisValue :type "Float (single-precision)"))
  ;[0 0 0] Rotates the character left/right by degree amount
  (if (>= (`KismetMathLibrary.Abs` AxisValue) (`self.Right Stick Threshold`))
    (`/Engine/EditorBlueprintResources/StandardMacros.DoOnce` false :!label _label
      (:`Completed`
        (`self.AddControllerYawInput` (* (`KismetMathLibrary.SignOfFloat` AxisValue) (`self.Snap Turn Angle`)))))
    (else
      (goto _label :!via `Reset`))))

(event `self.ReceiveTick`
  (params (DeltaSeconds :type "Float (single-precision)"))
  ;[0 0 0] Collider changes height with camera position
  (`CapsuleComponent.SetCapsuleHalfHeight` (`self.CapsuleComponent`) (stale `self.ReceiveBeginPlay` _output_get) true))

(event `self.ReceiveBeginPlay`
  (bind _returnvalue (`KismetMathLibrary.MakeTransform` (0.0 0.0 0.0)))
  (bind _capsulecomponent (`self.CapsuleComponent`))
  (`|ExecutionSequence`
    (:`then_0`
      ;[0 0 0] Collider changes height with camera position
      ;;[0 0 0] Halfway to the ground
      (bind _output_get (set `self.StartingCameraHeight` (.z (`SceneComponent.RelativeLocation` (`self.Camera`))))))
    (:`then_1`
      ;[0 0 0] Spawn and set controllers
      (`|ExecutionSequence`
        (:`then_0`
          (bind _returnvalue_2 (`|SpawnActorFromClass` "/Game/Blueprints/BP_MotionController.BP_MotionController_C" _returnvalue "AlwaysSpawn" "OverrideRootScale" self "Left" null))
          (bind _output_get_2 (set `self.Left Controller` _returnvalue_2))
          (`self.K2_AttachToComponent` _output_get_2 _capsulecomponent "None" "SnapToTarget" "SnapToTarget" "KeepWorld" false))
        (:`then_1`
          (bind _returnvalue_3 (`|SpawnActorFromClass` "/Game/Blueprints/BP_MotionController.BP_MotionController_C" _returnvalue "AlwaysSpawn" "OverrideRootScale" self "Right" null))
          (bind _output_get_3 (set `self.Right Controller` _returnvalue_3))
          (`self.K2_AttachToComponent` _output_get_3 _capsulecomponent "None" "SnapToTarget" "SnapToTarget" "KeepWorld" false))))))

(fn `UserConstructionScript`)