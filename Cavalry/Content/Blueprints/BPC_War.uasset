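; BPC_War is the Blueprint for War, an actor that buffs team shields when play begins.
; After the parent BeginPlay, it sets max and current shields to the same raised value on War, then on BPC_Death.
; Both targets come from GetActorOfClass lookups, so War finds itself by class and only one instance of each class is affected.
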(event `self.ReceiveBeginPlay`
  (`parent.ReceiveBeginPlay`)
  ;[0 0 0] Buffing Team shields
  (`|ExecutionSequence`
    (:`then_0`
      ;;[0.07227 0.07227 0.07227] War Shield buff
      (`GameplayStatics.GetActorOfClass` "BPC_War_C")
      (bind _output_get (set `self.MaxShields` 125))
      (set `self.CurrentShields` _output_get))
    (:`then_1`
      ;;[0.07227 0.07227 0.07227] Death Shield Buff
      (bind _returnvalue (`GameplayStatics.GetActorOfClass` "/Game/Blueprints/BPC_Death.BPC_Death_C"))
      (bind _output_get_2 (set `/Game/Blueprints/Base/BP_CavalryPlayerCharacter.MaxShields` 125 _returnvalue))
      (set `/Game/Blueprints/Base/BP_CavalryPlayerCharacter.CurrentShields` _output_get_2 _returnvalue))))

(fn `UserConstructionScript`
  (`parent.UserConstructionScript`))