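; Base VR firearm Blueprint that can be grabbed, dropped, fired, reloaded and switched between single and auto fire.
; Right-controller inputs drive firing, with auto looping while the trigger is held, plus firemode swapping and magazine ejection.
; Shots check load state, ammo and shotgun spent shells, then line-trace forward to damage enemies, without decrementing ammo.
; Reload-port overlap adds ammo from BP_Ammo_Base and attaches magazines, which eject as physics objects.
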(event `/Game/Blueprints/Interfaces/BPI_GrabbableObject.Pickup`
  (params (AttachTo :type "SceneComponent Object Reference"))
  ;[0 0 0] Grab Object
  (`PrimitiveComponent.SetSimulatePhysics` (`self.BaseWeaponSM`) false)
  (`SceneComponent.K2_AttachToComponent` (`self.DefaultSceneRoot`) AttachTo "None" "KeepWorld" "KeepWorld" "KeepWorld" false)
  (set `self.IsGrabbed` true))

(event `/Game/Blueprints/Interfaces/BPI_GrabbableObject.Drop`
  ;[0 0 0] Drop Object
  (`PrimitiveComponent.SetSimulatePhysics` (`self.BaseWeaponSM`) true)
  (`self.K2_DetachFromActor` "KeepWorld" "KeepWorld" "KeepWorld")
  (set `self.IsGrabbed` false))

(event `ShootFirearm`
  (bind _defaultsceneroot (`self.DefaultSceneRoot`))
  (bind _returnvalue (`SceneComponent.K2_GetComponentLocation` _defaultsceneroot))
  ;[0 0 0] Shooting
  (if (`self.IsGrabbed`)
    ;;[0.125 0.125 0.125] Are we loaded, have at least 1 ammo, no spent shells, and adding 1 spent shell if its a shotgun
    (if (`self.WeaponLoaded`)
      (if (< (`self.CurrentAmmo`) 1)
        _
        (elif (< (`self.SpentShells`) 1)
          (if (`|EnumEquality` (`self.LoadType`) "NewEnumerator1")
            (set `self.SpentShells` (+ (`self.SpentShells`) 1)))
          ;;[0.1302 0.1302 0.1302] Casting Ray
          (bind _outhit (`KismetSystemLibrary.LineTraceSingleForObjects` :`Start` _returnvalue :`End` (+ _returnvalue (* (`KismetMathLibrary.GetForwardVector` (`SceneComponent.K2_GetComponentRotation` _defaultsceneroot)) 200)) :`ObjectTypes` (`|MakeArray` "ObjectTypeQuery10" :!type "EObjectTypeQuery Enum") :`DrawDebugType` "ForOneFrame"))
          (bind (_bblockinghit _binitialoverlap _time _distance _location _impactpoint _normal _impactnormal _physmat _hitactor _hitcomponent) (`GameplayStatics.BreakHitResult` _outhit))
          ;;[0.1042 0.1042 0.1042] Did we hit an Enemy?
          (if (== (`PrimitiveComponent.GetCollisionObjectType` _hitcomponent) (enumliteral `EObjectTypeQuery` "ObjectTypeQuery10"))
            (message `/Game/Blueprints/Interfaces/BPI_Damage_Actor.TakeDamage` _hitactor (`self.DamageAmount`))))))))

(event `InputAction|TriggerRight`
  (params (Key :type "Key Structure"))
  ;[0 0 0] Player Input
  ;;[0.08854 0.08854 0.08854] Firing Input
  (:`Pressed`
    (set `self.TriggerPulled` true)
    (if (`self.IsGrabbed`)
      (switch `/Game/Blueprints/E_Firemodes` (`self.Firemode`)
        (:`NewEnumerator0`
          (`self.ShootFirearm` :!label _label))
        (:`NewEnumerator2`
          (while (`self.TriggerPulled`)
            (goto _label))))))
  (:`Released`
    (set `self.TriggerPulled` false)))

(event `InputAction|SecondaryButtonRight`
  (params (Key :type "Key Structure"))
  ;[0 0 0] Player Input
  ;;[0.09375 0.09375 0.09375] Swap Firemode Input
  (:`Pressed`
    (if (`self.IsGrabbed`)
      (`self.SwapFiremode`))))

(event `InputAction|PrimaryButtonRight`
  (params (Key :type "Key Structure"))
  ;[0 0 0] Player Input
  ;;[0.1354 0.1354 0.1354] Eject Ammo Input
  (:`Pressed`
    (if (`self.IsGrabbed`)
      (`self.EjectAmmo`))))

(event `SwapFiremode`
  ;[0 0 0] Swap Firemode
  (if (not (`self.TriggerPulled`))
    (switch `/Game/Blueprints/E_Firemodes` (`self.Firemode`)
      (:`NewEnumerator0`
        (if (`self.CanAutoFire`)
          (set `self.Firemode` "NewEnumerator2")))
      (:`NewEnumerator2`
        (if (`self.CanSingleFire`)
          (set `self.Firemode` "NewEnumerator0"))))))

(event `self.ReloadPortCollider.OnComponentBeginOverlap`
  (params (OverlappedComponent :type "PrimitiveComponent Object Reference") (OtherActor :type "Actor Object Reference") (OtherComp :type "PrimitiveComponent Object Reference") (OtherBodyIndex :type Integer) (bFromSweep :type Boolean) (SweepResult :type "HitResult Structure (by ref)"))
  ;[0 0 0] Reloading
  (if (not (`self.WeaponLoaded`))
    (bind _output_get (set `self.MagazineObj` OtherActor))
    (bind _asbp_ammo_base (cast `/Game/Blueprints/Base/BP_Ammo_Base` _output_get))
    (set `self.CurrentAmmo` (+ (`self.CurrentAmmo`) (`/Game/Blueprints/Base/BP_Ammo_Base.CurrentAmmo` _asbp_ammo_base)))
    (if (`|EnumEquality` (`self.LoadType`) "NewEnumerator0")
      (`self.K2_AttachToComponent` _output_get (`self.DefaultSceneRoot`) "None" "SnapToTarget" "SnapToTarget" "KeepWorld" false)
      (set `self.WeaponLoaded` true))))

(event `EjectAmmo`
  (bind _magazineobj (`self.MagazineObj`))
  ;[0 0 0] Eject Ammo
  (if (`self.TriggerPulled`)
    _
    (elif (`|EnumEquality` (`self.LoadType`) "NewEnumerator0")
      ;;[0.1094 0.1094 0.1094] Magazine
      (set `self.CurrentAmmo` 0)
      (`self.K2_DetachFromActor` _magazineobj "KeepWorld" "KeepWorld" "KeepWorld")
      (bind _asbp_ammo_base (cast `/Game/Blueprints/Base/BP_Ammo_Base` _magazineobj))
      (`PrimitiveComponent.SetSimulatePhysics` (`/Game/Blueprints/Base/BP_Ammo_Base.AmmoSM` _asbp_ammo_base) true)
      (set `self.WeaponLoaded` false))))

(fn `UserConstructionScript`)