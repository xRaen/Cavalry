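; Base VR player pawn for a cavalry character, with camera-relative movement, snap turning and a shield-based damage model.
; BeginPlay records the camera height that Tick applies as capsule half height, then spawns two motion controllers and a third-person model attached to the capsule.
; Damage that drives shields below zero adds a health hit and sets a timed recently-hit flag, while IncreaseShields adds shield and clears hits.
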(event `self.ReceiveTick`
  (params (DeltaSeconds :type "Float (single-precision)"))
  ;[0 0 0] Collider changes height with camera position
  (`CapsuleComponent.SetCapsuleHalfHeight` (`self.CapsuleComponent`) (stale `self.ReceiveBeginPlay` _output_get) true))

(event `self.ReceiveBeginPlay`
  (bind _returnvalue (`KismetMathLibrary.MakeTransform` (0.0 0.0 0.0)))
  (`|ExecutionSequence`
    (:`then_0`
      ;[0 0 0] Collider changes height with camera position
      ;;[0 0 0] Halfway to the ground
      (bind _output_get (set `self.StartingCameraHeight` (.z (`SceneComponent.RelativeLocation` (`self.Camera`))))))
    (:`then_1`
      ;[0 0 0] Spawn and set controllers
      (`|ExecutionSequence`
        (:`then_0`
          (bind _returnvalue_2 (`|SpawnActorFromClass` "/Game/Blueprints/BP_MotionController.BP_MotionController_C" _returnvalue "AlwaysSpawn" "OverrideRootScale" self "Left" null))
          (set `self.Left Controller` _returnvalue_2)
          (`self.K2_AttachToComponent` _returnvalue_2 (`self.CapsuleComponent`) "None" "SnapToTarget" "SnapToTarget" "KeepWorld" false))
        (:`then_1`
          (bind _returnvalue_3 (`|SpawnActorFromClass` "/Game/Blueprints/BP_MotionController.BP_MotionController_C" _returnvalue "AlwaysSpawn" "OverrideRootScale" self "Right" null))
          (set `self.Right Controller` _returnvalue_3)
          (`self.K2_AttachToComponent` _returnvalue_3 (`self.CapsuleComponent`) "None" "SnapToTarget" "SnapToTarget" "KeepWorld" false))))
    (:`then_2`
      ;[0 0 0] Spawn Third Person Model
      (bind _returnvalue_4 (`|SpawnActorFromClass` "/Game/Blueprints/Base/BP_3PCavalryCharacter.BP_3PCavalryCharacter_C" (`KismetMathLibrary.MakeTransform` (100.0 0.0 0.0)) "Undefined" "OverrideRootScale" self null))
      (bind _output_get_2 (set `self.3PModel` _returnvalue_4))
      (`self.K2_AttachToComponent` _output_get_2 (`self.CapsuleComponent`) "None" "SnapToTarget" "SnapToTarget" "KeepWorld" false))))

(event `/Game/Blueprints/Interfaces/BPI_DamageActor.TakeDamage`
  (params (DamageAmount :type Integer))
  (bind _currentshields (`self.CurrentShields`))
  ;[0 0 0] Taking Damage
  (set `self.CurrentShields` (- _currentshields DamageAmount))
  (if (< _currentshields 0)
    (set `self.CurrentShields` 0)
    (`/Engine/EditorBlueprintResources/StandardMacros.IncrementInt` (`self.HealthHits`)
      (:`  `
        (set `self.RecentlyHit` true)
        (`KismetSystemLibrary.K2_SetTimerDelegate` (delegate `ResetHitTimer`) 3.0)))))

(event `ResetHitTimer`
  ;[0 0 0] Taking Damage
  (set `self.RecentlyHit` false))

(fn `IncreaseShields`
  (params (Amount :type Integer))
  (set `self.CurrentShields` (+ Amount (`self.CurrentShields`)))
  (if (> (`self.HealthHits`) 0)
    (set `self.HealthHits` 0)))

(fn `Move`
  (params (`Scale Value` :type "Float (double-precision)"))
  ;[0.2471 0.2471 0.2471] Moves the character forward/backward
  (`self.AddMovementInput` (`SceneComponent.GetForwardVector` (`self.Camera`)) `Scale Value`))

(fn `Rotate`
  (params (`Scale Value` :type "Float (double-precision)"))
  ;[0 0 0] Rotates character based on degrees
  (if (>= (`KismetMathLibrary.Abs` `Scale Value`) (`self.Right Stick Threshold`))
    (`/Engine/EditorBlueprintResources/StandardMacros.DoOnce` false :!label _label
      (:`Completed`
        (`self.AddControllerYawInput` (* (`KismetMathLibrary.SignOfFloat` `Scale Value`) (`self.Snap Turn Angle`)))))
    (else
      (goto _label :!via `Reset`))))

(fn `Strafe`
  (params (`Scale Value` :type "Float (double-precision)"))
  ;[0.25 0.25 0.25] Moves the character left/right
  (`self.AddMovementInput` (`SceneComponent.GetRightVector` (`self.Camera`)) `Scale Value`))

(fn `UserConstructionScript`)