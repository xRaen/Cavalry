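; Base Blueprint for grabbable melee weapons that damage enemies on stab or slash.
; Pickup disables mesh physics and attaches the root to the supplied component keeping world transform, while Drop restores physics and detaches.
; Both events set IsGrabbed to false, including Pickup.
; DamageTrigger overlaps filter by the enemy collision object type and send a TakeDamage message with DamageAmount, with no swing-speed check.
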(event `/Game/Blueprints/Interfaces/BPI_GrabbableObject.Pickup`
  (params (AttachTo :type "SceneComponent Object Reference"))
  ;[0 0 0] Grab Object
  (`PrimitiveComponent.SetSimulatePhysics` (`self.MeleeSM`) false)
  (`SceneComponent.K2_AttachToComponent` (`self.DefaultSceneRoot`) AttachTo "None" "KeepWorld" "KeepWorld" "KeepWorld" false)
  (set `self.Is Grabbed` false))

(event `/Game/Blueprints/Interfaces/BPI_GrabbableObject.Drop`
  ;[0 0 0] Drop Object
  (`PrimitiveComponent.SetSimulatePhysics` (`self.MeleeSM`) true)
  (`self.K2_DetachFromActor` "KeepWorld" "KeepWorld" "KeepWorld")
  (set `self.Is Grabbed` false))

(event `self.DamageTrigger.OnComponentBeginOverlap`
  (params (OverlappedComponent :type "PrimitiveComponent Object Reference") (OtherActor :type "Actor Object Reference") (OtherComp :type "PrimitiveComponent Object Reference") (OtherBodyIndex :type Integer) (bFromSweep :type Boolean) (SweepResult :type "HitResult Structure (by ref)"))
  ;[0 0 0] Deal Damage on Stab/Slash
  ;;[0.1042 0.1042 0.1042] Did we hit an Enemy?
  (if (== (`PrimitiveComponent.GetCollisionObjectType` OtherComp) (enumliteral `EObjectTypeQuery` "ObjectTypeQuery10"))
    (message `/Game/Blueprints/Interfaces/BPI_Damage_Actor.TakeDamage` OtherActor (`self.DamageAmount`))))

(fn `UserConstructionScript`)