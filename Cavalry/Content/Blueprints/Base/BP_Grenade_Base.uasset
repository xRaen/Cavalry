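; BP_Grenade_Base is a base grenade Actor that can be grabbed, dropped and triggered on a countdown.
; Pickup disables mesh physics and attaches the root to the given component; Drop detaches, restores physics and enables Tick if the grenade is active.
; While active, Tick counts down from ActivationTime, then calls the empty ActivateGrenadeAbility event, resets the timer, deactivates and stops ticking.
; IsActive is never set to true here.
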(event `/Game/Blueprints/Interfaces/BPI_GrabbableObject.Pickup`
  (params (AttachTo :type "SceneComponent Object Reference"))
  ;[0 0 0] Grab Object
  (`PrimitiveComponent.SetSimulatePhysics` (`self.GrenadeSM`) false)
  (`SceneComponent.K2_AttachToComponent` (`self.DefaultSceneRoot`) AttachTo "None" "KeepWorld" "KeepWorld" "KeepWorld" false)
  (set `self.IsGrabbed` true))

(event `/Game/Blueprints/Interfaces/BPI_GrabbableObject.Drop`
  ;[0 0 0] Drop Object
  (`PrimitiveComponent.SetSimulatePhysics` (`self.GrenadeSM`) true)
  (`self.K2_DetachFromActor` "KeepWorld" "KeepWorld" "KeepWorld")
  (set `self.IsGrabbed` false)
  ;;[0.1042 0.1042 0.1042] Grenade is active and thrown
  (if (`self.IsActive`)
    (`self.SetActorTickEnabled` true)))

(event `self.ReceiveBeginPlay`
  ;[0 0 0] Grenade Activation Timer
  (set `self.CurrentActivationTime` (`self.ActivationTime`)))

(event `self.ReceiveTick`
  (params (DeltaSeconds :type "Float (single-precision)"))
  (bind _currentactivationtime (`self.CurrentActivationTime`))
  ;[0 0 0] Grenade Activation Timer
  (if (`self.IsActive`)
    (set `self.CurrentActivationTime` (- _currentactivationtime DeltaSeconds))
    (if (<= _currentactivationtime 0.0)
      (`self.ActivateGrenadeAbility`)
      (set `self.CurrentActivationTime` (`self.ActivationTime`))
      (set `self.IsActive` false)
      (`self.SetActorTickEnabled` false))))

(event `ActivateGrenadeAbility`)

(fn `UserConstructionScript`)