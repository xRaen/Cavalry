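; BP_MotionController is a VR hand actor that picks up and drops grabbable objects.
; Grab finds the nearest actor overlapping GrabCollider that implements BP_GrabbableObjectInterface, stores it as AttachedActor and sends it PickupMessage with the MotionController.
; Release sends DropMessage only if that actor is still attached to this controller, then clears the reference.
; The event graph holds no logic, and Grab and Release print debug strings.
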(event `self.GrabCollider.OnComponentBeginOverlap`
  (params (OverlappedComponent :type "PrimitiveComponent Object Reference") (OtherActor :type "Actor Object Reference") (OtherComp :type "PrimitiveComponent Object Reference") (OtherBodyIndex :type Integer) (bFromSweep :type Boolean) (SweepResult :type "HitResult Structure (by ref)")))

(fn `FindNearestGrabbableObject`
  (returns (NearestGrabbableObject :type "Actor Object Reference"))
  (locals (NearestOverlappingActor :type "Actor Object Reference") (NearestOverlap :type "Float (double-precision)"))
  (bind _grabcollider (`self.GrabCollider`))
  (for _array_element (`PrimitiveComponent.GetOverlappingActors` _grabcollider "/Script/Engine.Actor")
    ;[1 1 1] Does the object have the Grabbable Object interface on it?
    (if (`KismetSystemLibrary.DoesImplementInterface` _array_element "/Game/Blueprints/BP_GrabbableObjectInterface.BP_GrabbableObjectInterface_C")
      (bind _returnvalue (`KismetMathLibrary.VSize` (- (`self.K2_GetActorLocation` _array_element) (`SceneComponent.K2_GetComponentLocation` _grabcollider))))
      (if (< _returnvalue (`local.NearestOverlap`))
        (set `local.NearestOverlappingActor` _array_element)
        (set `local.NearestOverlap` _returnvalue))))
  (return (`local.NearestOverlappingActor`)))

(fn `Grab`
  (`KismetSystemLibrary.PrintString` "Grabbing :)")
  (bind _nearestgrabbableobject (`self.FindNearestGrabbableObject`))
  ;[1 1 0] Is this object a real object? (IDK I'm just doing it because Epic did it and they probably know a thing or two... maybe)
  (`/Engine/EditorBlueprintResources/StandardMacros.IsValid` _nearestgrabbableobject
    (:`Is Valid`
      (set `self.AttachedActor` _nearestgrabbableobject)
      (message `/Game/Blueprints/BP_GrabbableObjectInterface.Pickup` _nearestgrabbableobject (`self.MotionController`)))))

(fn `Release`
  (bind _attachedactor (`self.AttachedActor`))
  (`KismetSystemLibrary.PrintString` "I just released :)")
  ;[1 1 0] Is this object a real object? (IDK I'm just doing it because Epic did it and they probably know a thing or two... maybe)
  (`/Engine/EditorBlueprintResources/StandardMacros.IsValid` _attachedactor
    (:`Is Valid`
      (if (== (`SceneComponent.GetAttachParent` (`Actor.RootComponent` _attachedactor)) (`self.MotionController`))
        (message `/Game/Blueprints/BP_GrabbableObjectInterface.Drop` _attachedactor))
      (set `self.AttachedActor` null) ; Nulls Variable
    )))

(fn `UserConstructionScript`)