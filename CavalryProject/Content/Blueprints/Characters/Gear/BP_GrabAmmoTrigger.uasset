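; VR ammo pouch trigger that spawns a magazine or shotgun shell into the player's hand when grabbed.
; BeginPlay sets a carried count from the AmmoToSpawn type, and motion controller overlaps enable spawning through a hands-in-trigger counter.
; Grab spawns the matching ammo actor, attaches it via its GrabbableObjectSocket and decrements the count, which never limits spawning.
; End overlap decrements the hand counter for any actor, unlike begin overlap.
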(event `self.ReceiveBeginPlay`
  ;[0 0 0] Set how much ammo the player has on them
  (switch `/Game/Blueprints/Enums/E_LoadType` (`self.AmmoToSpawn`)
    (:`NewEnumerator0`
      (set `self.LoadTypeCount` 2))
    (:`NewEnumerator2`
      (set `self.LoadTypeCount` 4))
    (:`NewEnumerator3`
      (set `self.LoadTypeCount` 4))
    (:`NewEnumerator4`
      (set `self.LoadTypeCount` 4))
    (:`NewEnumerator1`
      (set `self.LoadTypeCount` 20))))

(event `self.Trigger.OnComponentBeginOverlap`
  (params (OverlappedComponent :type "PrimitiveComponent Object Reference") (OtherActor :type "Actor Object Reference") (OtherComp :type "PrimitiveComponent Object Reference") (OtherBodyIndex :type Integer) (bFromSweep :type Boolean) (SweepResult :type "HitResult Structure (by ref)"))
  ;[0 0 0] Player hand is inside Trigger
  (if (== OtherActor "/Game/VirtualRealityBP/Blueprints/BP_MotionController.BP_MotionController")
    (`KismetSystemLibrary.PrintString` "Owner hand is in Ammo Trigger")
    (set `self.canSpawn` true)
    (`/Engine/EditorBlueprintResources/StandardMacros.IncrementInt` (`self.NumberOfHandsInTrigger`))))

(event `self.Trigger.OnComponentEndOverlap`
  (params (OverlappedComponent :type "PrimitiveComponent Object Reference") (OtherActor :type "Actor Object Reference") (OtherComp :type "PrimitiveComponent Object Reference") (OtherBodyIndex :type Integer))
  (bind _numberofhandsintrigger (`self.NumberOfHandsInTrigger`))
  ;[0 0 0] Player hand has left trigger
  (`/Engine/EditorBlueprintResources/StandardMacros.DecrementInt` _numberofhandsintrigger
    (:`  `
      (if (not (> _numberofhandsintrigger 0))
        (set `self.canSpawn` false)))))

(event `/Game/Blueprints/Interfaces/BPI_GrabbableObj.Grab`
  (params (HandSocket :type Name) (AttachToMe :type "SceneComponent Object Reference") (Actor :type "Actor Object Reference"))
  (bind _returnvalue (`self.GetTransform` self))
  ;[0 0 0] Spawning and grabbing of Ammo
  (if (`self.canSpawn`)
    (switch `/Game/Blueprints/Enums/E_LoadType` (`self.AmmoToSpawn`)
      (:`NewEnumerator0`
        (bind _returnvalue_2 (`|SpawnActorFromClass` "/Game/Blueprints/Weapons/BPC_Pistol_Magazine.BPC_Pistol_Magazine_C" _returnvalue "AlwaysSpawn" "OverrideRootScale" null 1 null))
        (bind _output_get (set `self.SpawnedAmmo` _returnvalue_2))
        (`/Engine/EditorBlueprintResources/StandardMacros.DecrementInt` (`self.LoadTypeCount`)
          (:`  `
            (`/Game/Blueprints/GrabbableObjectSocket.Grab` (`self.GetComponentByClass` _output_get "/Game/Blueprints/GrabbableObjectSocket.GrabbableObjectSocket_C") (`/Game/Blueprints/Weapons/BP_AmmoBase.Ammo_SM` _returnvalue_2) _returnvalue_2 HandSocket AttachToMe))))
      (:`NewEnumerator2`
        (bind _returnvalue_3 (`|SpawnActorFromClass` "/Game/Blueprints/Weapons/BPC_Rifle_Magazine.BPC_Rifle_Magazine_C" _returnvalue "AlwaysSpawn" "OverrideRootScale" null 1 null))
        (bind _output_get_2 (set `self.SpawnedAmmo` _returnvalue_3))
        (`/Engine/EditorBlueprintResources/StandardMacros.DecrementInt` (`self.LoadTypeCount`)
          (:`  `
            (`/Game/Blueprints/GrabbableObjectSocket.Grab` (`self.GetComponentByClass` _output_get_2 "/Game/Blueprints/GrabbableObjectSocket.GrabbableObjectSocket_C") (`/Game/Blueprints/Weapons/BP_AmmoBase.Ammo_SM` _returnvalue_3) _returnvalue_3 HandSocket AttachToMe))))
      (:`NewEnumerator3`
        (bind _returnvalue_4 (`|SpawnActorFromClass` "/Game/Blueprints/Weapons/BPC_DMR_Magazine.BPC_DMR_Magazine_C" _returnvalue "AlwaysSpawn" "OverrideRootScale" null 1 null))
        (bind _output_get_3 (set `self.SpawnedAmmo` _returnvalue_4))
        (`/Engine/EditorBlueprintResources/StandardMacros.DecrementInt` (`self.LoadTypeCount`)
          (:`  `
            (`/Game/Blueprints/GrabbableObjectSocket.Grab` (`self.GetComponentByClass` _output_get_3 "/Game/Blueprints/GrabbableObjectSocket.GrabbableObjectSocket_C") (`/Game/Blueprints/Weapons/BP_AmmoBase.Ammo_SM` _returnvalue_4) _returnvalue_4 HandSocket AttachToMe))))
      (:`NewEnumerator4`
        (bind _returnvalue_5 (`|SpawnActorFromClass` "/Game/Blueprints/Weapons/BPC_SMG_Magazine.BPC_SMG_Magazine_C" _returnvalue "AlwaysSpawn" "OverrideRootScale" null 1 null))
        (bind _output_get_4 (set `self.SpawnedAmmo` _returnvalue_5))
        (`/Engine/EditorBlueprintResources/StandardMacros.DecrementInt` (`self.LoadTypeCount`)
          (:`  `
            (`/Game/Blueprints/GrabbableObjectSocket.Grab` (`self.GetComponentByClass` _output_get_4 "/Game/Blueprints/GrabbableObjectSocket.GrabbableObjectSocket_C") (`/Game/Blueprints/Weapons/BP_AmmoBase.Ammo_SM` _returnvalue_5) _returnvalue_5 HandSocket AttachToMe))))
      (:`NewEnumerator1`
        (bind _returnvalue_6 (`|SpawnActorFromClass` "/Game/Blueprints/Weapons/BPC_Shotgun_Shell.BPC_Shotgun_Shell_C" _returnvalue "AlwaysSpawn" "OverrideRootScale" null 1 null))
        (bind _output_get_5 (set `self.SpawnedAmmo` _returnvalue_6))
        (`/Engine/EditorBlueprintResources/StandardMacros.DecrementInt` (`self.LoadTypeCount`)
          (:`  `
            (`/Game/Blueprints/GrabbableObjectSocket.Grab` (`self.GetComponentByClass` _output_get_5 "/Game/Blueprints/GrabbableObjectSocket.GrabbableObjectSocket_C") (`/Game/Blueprints/Weapons/BP_AmmoBase.Ammo_SM` _returnvalue_6) _returnvalue_6 HandSocket AttachToMe)))))))

(fn `UserConstructionScript`)