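; BP_CavalryController is the VR player controller that routes motion controller input to the character it possesses.
; On BeginPlay it stores the possessed pawn as one of the Conquest, War, Death or Famine characters, or the base player character.
; Thumbsticks drive movement, strafing and rotation, while grip inputs grab and release through each hand.
; Triggers and buttons message the character's gear for per-hand firing, magazine release, firemode and tool toggling, plus night vision.
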(event `self.ReceiveBeginPlay`
  (bind _returnvalue (`self.K2_GetPawn`))
  ;[1 1 1] Grabbing the character that this controller possesses
  (`|ExecutionSequence`
    (:`then_0`
      (bind _asbpc_conquest (cast `/Game/Blueprints/Characters/BPC_Conquest` _returnvalue))
      (`/Engine/EditorBlueprintResources/StandardMacros.IsValid` _asbpc_conquest
        (:`Is Valid`
          (set `self.possessedCharacter` _asbpc_conquest))))
    (:`then_1`
      (bind _asbpc_war (cast `/Game/Blueprints/Characters/BPC_War` _returnvalue))
      (`/Engine/EditorBlueprintResources/StandardMacros.IsValid` _asbpc_war
        (:`Is Valid`
          (set `self.possessedCharacter` _asbpc_war))))
    (:`then_2`
      (bind _asbpc_death (cast `/Game/Blueprints/Characters/BPC_Death` _returnvalue))
      (`/Engine/EditorBlueprintResources/StandardMacros.IsValid` _asbpc_death
        (:`Is Valid`
          (set `self.possessedCharacter` _asbpc_death))))
    (:`then_3`
      (bind _asbpc_famine (cast `/Game/Blueprints/Characters/BPC_Famine` _returnvalue))
      (`/Engine/EditorBlueprintResources/StandardMacros.IsValid` _asbpc_famine
        (:`Is Valid`
          (set `self.possessedCharacter` _asbpc_famine))))
    (:`then_4`
      (bind _asbp_player_character_base (cast `/Game/Blueprints/Characters/BP_PlayerCharacter_Base` _returnvalue))
      (`/Engine/EditorBlueprintResources/StandardMacros.IsValid` _asbp_player_character_base
        (:`Is Valid`
          (set `self.possessedCharacter` _asbp_player_character_base))))))

(event `InputAxis|MotionControllerThumbLeft_Y`
  (params (AxisValue :type "Float (single-precision)"))
  ;[1 1 1] Player Input
  ;;[0.1095 0.1095 0.1095] Forward/Backward Movement
  (`/Game/Blueprints/Characters/BP_PlayerCharacter_Base.Movement` (`self.possessedCharacter`) AxisValue))

(event `InputAxis|MotionControllerThumbLeft_X`
  (params (AxisValue :type "Float (single-precision)"))
  ;[1 1 1] Player Input
  ;;[0.1095 0.1095 0.1095] Left/Right Movement
  (`/Game/Blueprints/Characters/BP_PlayerCharacter_Base.Strafe` (`self.possessedCharacter`) AxisValue))

(event `InputAction|GrabLeft`
  (params (Key :type "Key Structure"))
  (bind _left_controller (`/Game/Blueprints/Characters/BP_PlayerCharacter_Base.Left Controller` (`self.possessedCharacter`)))
  ;[1 1 1] Player Input
  ;;[0.1095 0.1095 0.1095] Left Grabbing
  (:`Pressed`
    (`/Game/VirtualRealityBP/Blueprints/BP_MotionController.GrabActor` _left_controller))
  (:`Released`
    (`/Game/VirtualRealityBP/Blueprints/BP_MotionController.ReleaseActor` _left_controller)))

(event `InputAxis|MotionControllerThumbRight_X`
  (params (AxisValue :type "Float (single-precision)"))
  ;[1 1 1] Player Input
  ;;[0.1095 0.1095 0.1095] Rotation
  (`/Game/Blueprints/Characters/BP_PlayerCharacter_Base.Rotation` (`self.possessedCharacter`) AxisValue))

(event `InputAction|GrabRight`
  (params (Key :type "Key Structure"))
  (bind _right_controller (`/Game/Blueprints/Characters/BP_PlayerCharacter_Base.Right Controller` (`self.possessedCharacter`)))
  ;[1 1 1] Player Input
  ;;[0.1095 0.1095 0.1095] Right Grabbing
  (:`Pressed`
    (`/Game/VirtualRealityBP/Blueprints/BP_MotionController.GrabActor` _right_controller))
  (:`Released`
    (`/Game/VirtualRealityBP/Blueprints/BP_MotionController.ReleaseActor` _right_controller)))

(event `InputAction|PrimaryTriggerLeft`
  (params (Key :type "Key Structure"))
  (bind _playergear (`/Game/Blueprints/Characters/BP_PlayerCharacter_Base.PlayerGear` (`self.possessedCharacter`)))
  ;[1 1 1] Player Input
  ;;[0.1095 0.1095 0.1095] Fire Weapon Left
  (:`Pressed`
    (message `/Game/Blueprints/Interfaces/BPI_WeaponControls.Shoot` (`/Game/Blueprints/Characters/Gear/BP_PlayerGear.MainWeapon` _playergear) "NewEnumerator1")
    (message `/Game/Blueprints/Interfaces/BPI_WeaponControls.Shoot` (`/Game/Blueprints/Characters/Gear/BP_PlayerGear.Pistol` _playergear) "NewEnumerator1")))

(event `InputAction|PrimaryButtonRight`
  (params (Key :type "Key Structure"))
  (bind _playergear (`/Game/Blueprints/Characters/BP_PlayerCharacter_Base.PlayerGear` (`self.possessedCharacter`)))
  (bind _tool (`/Game/Blueprints/Characters/Gear/BP_PlayerGear.Tool` _playergear))
  ;[1 1 1] Player Input
  ;;[0.1095 0.1095 0.1095] Release Weapon Magazine / Activate Tool
  (:`Pressed`
    (message `/Game/Blueprints/Interfaces/BPI_WeaponControls.ReleaseMagazine` (`/Game/Blueprints/Characters/Gear/BP_PlayerGear.MainWeapon` _playergear))
    (message `/Game/Blueprints/Interfaces/BPI_WeaponControls.ReleaseMagazine` (`/Game/Blueprints/Characters/Gear/BP_PlayerGear.Pistol` _playergear))
    (if (`/Game/Blueprints/Tools/BP_Tool_Base.toolActivated` _tool)
      (message `/Game/Blueprints/Interfaces/BPI_ToolControls.ActivateTool` _tool false)
      (else
        (message `/Game/Blueprints/Interfaces/BPI_ToolControls.ActivateTool` _tool true)))))

(event `InputAction|PrimaryTriggerRight`
  (params (Key :type "Key Structure"))
  (bind _playergear (`/Game/Blueprints/Characters/BP_PlayerCharacter_Base.PlayerGear` (`self.possessedCharacter`)))
  ;[1 1 1] Player Input
  ;;[0.1095 0.1095 0.1095] Fire Weapon Right
  (:`Pressed`
    (message `/Game/Blueprints/Interfaces/BPI_WeaponControls.Shoot` (`/Game/Blueprints/Characters/Gear/BP_PlayerGear.MainWeapon` _playergear) "NewEnumerator0")
    (message `/Game/Blueprints/Interfaces/BPI_WeaponControls.Shoot` (`/Game/Blueprints/Characters/Gear/BP_PlayerGear.Pistol` _playergear) "NewEnumerator0")))

(event `InputAction|SecondaryButtonRight`
  (params (Key :type "Key Structure"))
  ;[1 1 1] Player Input
  ;;[0.1095 0.1095 0.1095] Change Weapon Firemode
  (:`Pressed`
    (message `/Game/Blueprints/Interfaces/BPI_WeaponControls.ChangeFiremode` (`/Game/Blueprints/Characters/Gear/BP_PlayerGear.MainWeapon` (`/Game/Blueprints/Characters/BP_PlayerCharacter_Base.PlayerGear` (`self.possessedCharacter`))))))

(event `InputAction|PrimaryButtonLeft`
  (params (Key :type "Key Structure"))
  (:`Pressed`
    (`/Game/Blueprints/Characters/BP_PlayerCharacter_Base.Night Vision Trigger` (`self.possessedCharacter`))))

(fn `UserConstructionScript`)