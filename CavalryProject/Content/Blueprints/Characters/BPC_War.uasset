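; BPC_War is the War character Blueprint, whose shield buff ability applies to War, Death, Famine and Conquest.
; After the parent BeginPlay, a sequence finds the first actor of each of those four classes and, if valid, sets its MaxShields to one fixed value.
; Nodes that would copy MaxShields into CurrentShields are unconnected, so the buff leaves current shields untouched.
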(event `self.ReceiveBeginPlay`
  ;[1 1 1] War shield buff ability
  (`parent.ReceiveBeginPlay`)
  (`|ExecutionSequence`
    (:`then_0`
      (bind _returnvalue (`GameplayStatics.GetActorOfClass` "BPC_War_C"))
      (`/Engine/EditorBlueprintResources/StandardMacros.IsValid` _returnvalue
        (:`Is Valid`
          (bind _output_get (set `/Game/Blueprints/Characters/BP_PlayerCharacter_Base.maxShields` 150 _returnvalue)))))
    (:`then_1`
      (bind _returnvalue_2 (`GameplayStatics.GetActorOfClass` "/Game/Blueprints/Characters/BPC_Death.BPC_Death_C"))
      (`/Engine/EditorBlueprintResources/StandardMacros.IsValid` _returnvalue_2
        (:`Is Valid`
          (bind _output_get_2 (set `/Game/Blueprints/Characters/BP_PlayerCharacter_Base.maxShields` 150 _returnvalue_2)))))
    (:`then_2`
      (bind _returnvalue_3 (`GameplayStatics.GetActorOfClass` "/Game/Blueprints/Characters/BPC_Famine.BPC_Famine_C"))
      (`/Engine/EditorBlueprintResources/StandardMacros.IsValid` _returnvalue_3
        (:`Is Valid`
          (bind _output_get_3 (set `/Game/Blueprints/Characters/BP_PlayerCharacter_Base.maxShields` 150 _returnvalue_3)))))
    (:`then_3`
      (bind _returnvalue_4 (`GameplayStatics.GetActorOfClass` "/Game/Blueprints/Characters/BPC_Conquest.BPC_Conquest_C"))
      (`/Engine/EditorBlueprintResources/StandardMacros.IsValid` _returnvalue_4
        (:`Is Valid`
          (bind _output_get_4 (set `/Game/Blueprints/Characters/BP_PlayerCharacter_Base.maxShields` 150 _returnvalue_4)))))))

(fn `UserConstructionScript`
  (`parent.UserConstructionScript`))