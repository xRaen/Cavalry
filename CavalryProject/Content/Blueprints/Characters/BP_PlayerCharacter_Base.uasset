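; Base VR player character for a Horsemen game, spawning and attaching two motion controllers, horseman-specific gear and a camera-mounted HUD.
; Each tick aligns gear to headset yaw and moves the capsule under the camera, counter-offsetting the VR origin.
; Damage drains shields, then counts health hits with brief invulnerability until death disables grabbing.
; Also provides camera-relative movement, snap turning, KAT treadmill locomotion and a Famine-dependent night vision toggle.
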(event `self.ReceiveBeginPlay`
  (bind _returnvalue (`KismetMathLibrary.MakeTransform` (0.0 0.0 0.0)))
  (`|ExecutionSequence`
    (:`then_0`
      ;[1 1 1] Setup Player Height for Each HMD [Oculus, Odyssey, SteamVR]
      (switch `name` (`HeadMountedDisplayFunctionLibrary.GetHMDDeviceName`)
        (:`Oculus HMD`
          _)
        (:`Windows Mixed Reality`
          _))
      (`HeadMountedDisplayFunctionLibrary.SetTrackingOrigin` "Floor"))
    (:`then_1`
      (`|ExecutionSequence`
        (:`then_0`
          ;[1 1 1] Motion Controller Spawn and Attach
          (bind _returnvalue_2 (`|SpawnActorFromClass` "/Game/VirtualRealityBP/Blueprints/BP_MotionController.BP_MotionController_C" _returnvalue "AlwaysSpawn" "OverrideRootScale" self "Left" null))
          (set `self.Left Controller` _returnvalue_2)
          (`self.K2_AttachToComponent` _returnvalue_2 (`self.VR Origin`) "None" "SnapToTarget" "SnapToTarget" "KeepWorld" false))
        (:`then_1`
          (bind _returnvalue_3 (`|SpawnActorFromClass` "/Game/VirtualRealityBP/Blueprints/BP_MotionController.BP_MotionController_C" _returnvalue "AlwaysSpawn" "OverrideRootScale" self "Right" null))
          (set `self.Right Controller` _returnvalue_3)
          (`self.K2_AttachToComponent` _returnvalue_3 (`self.VR Origin`) "None" "SnapToTarget" "SnapToTarget" "KeepWorld" false))
        (:`then_2`
          ;[1 1 1] Gear Spawning (default horseman is War)
          (bind _returnvalue_4 (`|SpawnActorFromClass` "/Game/Blueprints/Characters/Gear/BP_PlayerGear.BP_PlayerGear_C" (`KismetMathLibrary.MakeTransform` (0.0 0.0 0.0)) "AlwaysSpawn" "OverrideRootScale" self (`self.Horseman to Spawn For`) null))
          (bind _output_get (set `self.PlayerGear` _returnvalue_4))
          (`self.K2_AttachToComponent` _output_get (`self.GearLoction`) "None" "SnapToTarget" "SnapToTarget" "SnapToTarget" false)
          (set `/Game/Blueprints/Characters/Gear/BP_PlayerGear.AttachedPlayer` self _returnvalue_4))
        (:`then_3`
          ;[1 1 1] HUD Spawning
          (bind _returnvalue_5 (`|SpawnActorFromClass` "/Game/HUD/Widgets/Damage_Display/BP_HorsemenHUD.BP_HorsemenHUD_C" (`KismetMathLibrary.MakeTransform` (0.0 0.0 0.0) (struct) (0.1 0.1 0.1)) "AlwaysSpawn" "OverrideRootScale" self null))
          (bind _output_get_2 (set `self.WidgetHandler` _returnvalue_5))
          (`self.K2_AttachToComponent` _output_get_2 (`self.Camera`) "None" "KeepRelative" "KeepRelative" "KeepRelative" false))))
    (:`then_2`
      (set `PostProcessComponent.bEnabled` false (`self.Night Vision PP`))
      (set `PostProcessComponent.bEnabled` false (`self.PlayerDeath`)))
    (:`then_3`
      (`HeadMountedDisplayFunctionLibrary.SetTrackingOrigin` "Floor"))))

(event `/Game/Blueprints/Interfaces/BPI_TakeDamage.TakeDamage`
  (params (DamageAmount :type Integer))
  (bind _currentshields (`self.currentShields`))
  ;[1 1 1] Taking Damage
  (if (not (`self.recentlyHit`))
    (set `self.currentShields` (- _currentshields DamageAmount))
    (if (<= _currentshields 0)
      (set `self.currentShields` 0)
      (`/Engine/EditorBlueprintResources/StandardMacros.IncrementInt` (`self.healthHits`)
        (:`  `
          (set `self.recentlyHit` true)
          (`self.ResetShieldPercentage`)
          (`KismetSystemLibrary.K2_SetTimerDelegate` (delegate `ResetHitTimer`) 3.0)
          ;[1 1 1] Should player be dead?
          (if (>= (`self.healthHits`) (`self.maxHealthHits`))
            (`self.Death`)))))))

(event `ResetHitTimer`
  ;[1 1 1] Taking Damage
  (set `self.recentlyHit` false))

(event `Death`
  (bind _left_controller (`self.Left Controller`))
  (bind _right_controller (`self.Right Controller`))
  ;[1 1 1] Player Death
  (`PrimitiveComponent.SetCollisionEnabled` (`/Game/VirtualRealityBP/Blueprints/BP_MotionController.GrabSphere` _left_controller) "NoCollision")
  (`/Game/VirtualRealityBP/Blueprints/BP_MotionController.ReleaseActor` _left_controller)
  (`PrimitiveComponent.SetCollisionEnabled` (`/Game/VirtualRealityBP/Blueprints/BP_MotionController.GrabSphere` _right_controller) "NoCollision")
  (`/Game/VirtualRealityBP/Blueprints/BP_MotionController.ReleaseActor` _right_controller)
  (set `PostProcessComponent.bEnabled` false (`self.Night Vision PP`))
  (set `PostProcessComponent.bEnabled` true (`self.PlayerDeath`))
  (`KismetArrayLibrary.Array_Remove` (`self.Tags`))
  (`self.RemoveAsTarget`))

(event `Initialize Capsule Height`
  ;[1 1 1] Grabbing Capsule Half-Height
)

(event `Night Vision Trigger`
  (bind _night_vision_pp (`self.Night Vision PP`))
  ;[1 1 1] Famine Ability: Night vision
  (bind _returnvalue (`GameplayStatics.GetActorOfClass` "/Game/Blueprints/Characters/BPC_Famine.BPC_Famine_C"))
  (if (`KismetSystemLibrary.IsValid` _returnvalue)
    (`KismetSystemLibrary.PrintString` "Night Vision Trigger Success: Famine in Scene" true true (struct :`G` 1.0 :`B` 0.193288 :`A` 1.0))
    (`/Engine/EditorBlueprintResources/StandardMacros.FlipFlop`
      (:`A`
        (set `PostProcessComponent.bEnabled` true _night_vision_pp)
        (`KismetSystemLibrary.PrintString` "Night Vision Trigger ON" true true (struct :`G` 1.0 :`B` 0.193288 :`A` 1.0)))
      (:`B`
        (set `PostProcessComponent.bEnabled` false _night_vision_pp)
        (`KismetSystemLibrary.PrintString` "Night Vision Trigger OFF" true true (struct :`R` 1.0 :`A` 1.0))))
    (else
      (`KismetSystemLibrary.PrintString` "Night Vision Trigger Failure: Famine not in Scene" true true (struct :`R` 1.0 :`A` 1.0)))))

(event `self.ReceiveTick`
  (params (DeltaSeconds :type "Float (single-precision)"))
  (bind _gearlocationbase (`self.GearLocationBase`))
  (bind (_returnvalue_roll _returnvalue_pitch _returnvalue_yaw) (`KismetMathLibrary.BreakRotator` (`SceneComponent.K2_GetComponentRotation` (`self.Camera`))))
  (`|ExecutionSequence`
    (:`then_0`
      ;[1 1 1] Gear Rotation
      (`SceneComponent.K2_SetWorldRotation` _gearlocationbase (`KismetMathLibrary.MakeRotator` 0.0 0.0 _returnvalue_yaw) false false)
      (`SceneComponent.K2_SetWorldLocation` _gearlocationbase (`SceneComponent.K2_GetComponentLocation` (`self.Camera`)) false false))
    (:`then_1`
      (`self.UpdatePlayerCollisionPosition`))))

(event `ResetShieldPercentage`
  ;[1 1 1] Shield Percentage Reset
  (bind _asbp_magnetic_placement (cast `/Game/Blueprints/Tools/BP_MagneticPlacement` (`ChildActorComponent.ChildActor` (`/Game/Blueprints/Characters/Gear/BP_PlayerGear.Magnet 8` (`self.PlayerGear`)))))
  (bind _asbpc_shield_recharger (cast `/Game/Blueprints/Tools/BPC_ShieldRecharger` (`/Game/Blueprints/Tools/BP_MagneticPlacement.AttachedObject` _asbp_magnetic_placement)))
  (`TextRenderComponent.K2_SetText` (`/Game/Blueprints/Tools/BPC_ShieldRecharger.TextRender` _asbpc_shield_recharger) (`KismetTextLibrary.Conv_StringToText` (`KismetStringLibrary.Concat_StrStr` (`KismetStringLibrary.Conv_IntToString` (`KismetMathLibrary.FTrunc` (* (/ (`KismetMathLibrary.Conv_IntToDouble` (`self.currentShields`)) (`KismetMathLibrary.Conv_IntToDouble` (`self.maxShields`))) 100.0))) "%"))))

(event `UpdatePlayerCollisionPosition`
  (bind (_returnvalue_x _returnvalue_y) (`KismetMathLibrary.BreakVector` (- (`SceneComponent.K2_GetComponentLocation` (`self.Camera`)) (`SceneComponent.K2_GetComponentLocation` (`self.CapsuleComponent`)))))
  ;[0 0 0] Player collision position updating
  (`self.K2_AddActorWorldOffset` (`KismetMathLibrary.MakeVector` _returnvalue_x _returnvalue_y) true)
  (`SceneComponent.K2_AddWorldOffset` (`self.VR Origin`) (`KismetMathLibrary.NegateVector` (`KismetMathLibrary.MakeVector` _returnvalue_x _returnvalue_y)) false false))

(fn `KATMovement`
  (params (BodyYawVar :type "Float (double-precision)"))
  (bind (_returnvalue_x _returnvalue_y) (`KismetMathLibrary.BreakVector` (`self.GetActorForwardVector` self)))
  (`SceneComponent.K2_SetRelativeRotation` (`self.CapsuleComponent`) (`KismetMathLibrary.MakeRotator` 0.0 0.0 (- (`KatDataPlugin4BPBPLibrary.BodyYaw_KatDataPlugin4BP`) BodyYawVar)) false false)
  (`self.K2_AddActorWorldOffset` (* (`KismetMathLibrary.MakeVector` _returnvalue_x _returnvalue_y) (* (* (* (`KatDataPlugin4BPBPLibrary.MoveDirection_KatDataPlugin4BP`) (`KatDataPlugin4BPBPLibrary.IsMoving_KatDataPlugin4BP`)) (`KatDataPlugin4BPBPLibrary.WalkPower_KatDataPlugin4BP`)) (`CharacterMovementComponent.MaxWalkSpeed` (`self.CharacterMovement`)))) true))

(fn `Movement`
  (params (Value :type "Float (double-precision)"))
  ;[1 1 1] Forward and Backward Movement
  (`self.AddMovementInput` (`SceneComponent.GetForwardVector` (`self.Camera`)) Value))

(fn `Rotation`
  (params (value :type "Float (double-precision)"))
  ;[1 1 1] Rotation
  (`self.K2_AddActorWorldRotation` (`KismetMathLibrary.MakeRotator` 0.0 0.0 (* (`KismetMathLibrary.SignOfFloat` value) (`self.Snap Rotation Degrees`)))))

(fn `Strafe`
  (params (value :type "Float (double-precision)"))
  ;[1 1 1] Strafe Movement Input
  (`self.AddMovementInput` (`SceneComponent.GetRightVector` (`self.Camera`)) value))

(fn `UserConstructionScript`)