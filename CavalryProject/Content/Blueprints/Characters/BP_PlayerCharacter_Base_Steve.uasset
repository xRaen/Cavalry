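; Base VR player character with camera-relative movement, strafing and deadzoned snap or smooth turning.
; On BeginPlay it sets floor tracking for Oculus and Windows MR, spawns and attaches both motion controllers and horseman-specific gear, and traces down for an HMD floor origin.
; Tick uses that origin and the camera to keep the gear base following the head, pitch zeroed.
; Damage drains shields, then counts timer-gated health hits toward a print-only death.
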(event `self.ReceiveBeginPlay`
  (bind _returnvalue (`KismetMathLibrary.MakeTransform` (0.0 0.0 0.0)))
  (`|ExecutionSequence`
    (:`then_0`
      ;[1 1 1] Setup Player Height for Each HMD [Oculus, Odyssey, SteamVR]
      (switch `name` (`HeadMountedDisplayFunctionLibrary.GetHMDDeviceName`)
        (:`Oculus HMD`
          _)
        (:`Windows Mixed Reality`
          _))
      (`HeadMountedDisplayFunctionLibrary.SetTrackingOrigin` "Floor"))
    (:`then_1`
      (`|ExecutionSequence`
        (:`then_0`
          ;[1 1 1] Motion Controller Spawn and Attach
          (bind _returnvalue_2 (`|SpawnActorFromClass` "/Game/VirtualRealityBP/Blueprints/BP_MotionController.BP_MotionController_C" _returnvalue "AlwaysSpawn" "OverrideRootScale" self "Left" null))
          (set `self.Left Controller` _returnvalue_2)
          (`self.K2_AttachToComponent` _returnvalue_2 (`self.CapsuleComponent`) "None" "SnapToTarget" "SnapToTarget" "KeepWorld" false))
        (:`then_1`
          (bind _returnvalue_3 (`|SpawnActorFromClass` "/Game/VirtualRealityBP/Blueprints/BP_MotionController.BP_MotionController_C" _returnvalue "AlwaysSpawn" "OverrideRootScale" self "Right" null))
          (set `self.Right Controller` _returnvalue_3)
          (`self.K2_AttachToComponent` _returnvalue_3 (`self.CapsuleComponent`) "None" "SnapToTarget" "SnapToTarget" "KeepWorld" false))
        (:`then_2`
          ;[1 1 1] Gear Spawning (default horseman is War)
          (bind _returnvalue_4 (`|SpawnActorFromClass` "/Game/Blueprints/Characters/Gear/BP_PlayerGear.BP_PlayerGear_C" (`KismetMathLibrary.MakeTransform` (0.0 0.0 0.0)) "AlwaysSpawn" "OverrideRootScale" self (`self.Horseman to Spawn For`) null))
          (bind _output_get (set `self.PlayerGear` _returnvalue_4))
          (`self.K2_AttachToComponent` _output_get (`self.GearLoction`) "None" "SnapToTarget" "SnapToTarget" "SnapToTarget" false))))
    (:`then_2`
      (`self.Initialize Capsule Height`))
    (:`then_3`
      (`self.Calibrate HMD Floor Position`))))

(event `/Game/Blueprints/Interfaces/BPI_TakeDamage.TakeDamage`
  (params (DamageAmount :type Integer))
  (bind _currentshields (`self.currentShields`))
  ;[1 1 1] Taking Damage
  (if (not (`self.recentlyHit`))
    (set `self.currentShields` (- _currentshields DamageAmount))
    (if (<= _currentshields 0)
      (set `self.currentShields` 0)
      (`/Engine/EditorBlueprintResources/StandardMacros.IncrementInt` (`self.healthHits`)
        (:`  `
          (set `self.recentlyHit` true)
          (`KismetSystemLibrary.K2_SetTimerDelegate` (delegate `ResetHitTimer`) 3.0)
          ;[1 1 1] Should player be dead?
          (if (>= (`self.healthHits`) (`self.maxHealthHits`))
            (`self.Death`)))))))

(event `ResetHitTimer`
  ;[1 1 1] Taking Damage
  (set `self.recentlyHit` false))

(event `Death`
  ;[1 1 1] Player Death
  (`KismetSystemLibrary.PrintString` "You are dead :)"))

(event `Initialize Capsule Height`
  ;[1 1 1] Grabbing Capsule Half-Height
)

(event `Set Capsule Height`
  (bind _returnvalue (+ (/ 0.0 2.0) 5.0))
  (`CapsuleComponent.SetCapsuleHalfHeight` (`self.CapsuleComponent`) _returnvalue true)
  (`SceneComponent.K2_AddRelativeLocation` (`self.Camera`) (`KismetMathLibrary.MakeVector` 0.0 0.0 (- (`self.Previous Capsule Half-Height`) _returnvalue)) false false)
  (set `self.Previous Capsule Half-Height` _returnvalue))

(event `self.ReceiveTick`
  (params (DeltaSeconds :type "Float (single-precision)"))
  (bind _camera (`self.Camera`))
  (bind _gearlocationbase (`self.GearLocationBase`))
  (bind (_relativerotation_roll _relativerotation_pitch _relativerotation_yaw) (`KismetMathLibrary.BreakRotator` (`SceneComponent.RelativeRotation` _gearlocationbase)))
  ;[0 0 0] Gear Rotation
  (`SceneComponent.K2_SetWorldRotation` _gearlocationbase (`KismetMathLibrary.MakeRotFromXZ` (`SceneComponent.GetForwardVector` _camera) (- (`SceneComponent.K2_GetComponentLocation` _camera) (+ (`self.HMD_Origin`) (`SceneComponent.K2_GetComponentLocation` (`self.CapsuleComponent`))))) false false)
  (`SceneComponent.K2_SetWorldLocation` _gearlocationbase (`SceneComponent.K2_GetComponentLocation` (`self.Camera`)) false false)
  (`SceneComponent.K2_SetRelativeRotation` _gearlocationbase (`KismetMathLibrary.MakeRotator` _relativerotation_roll 0.0 _relativerotation_yaw) false false))

(event `Calibrate HMD Floor Position`
  (bind _returnvalue (`SceneComponent.K2_GetComponentLocation` (`self.Camera`)))
  ;[0 0 0] capture the initial HMD position towards the ground
  (bind _outhit (`KismetSystemLibrary.LineTraceSingleForObjects` _returnvalue (+ _returnvalue (0.0 0.0 -1000.0)) (`|MakeArray` "ObjectTypeQuery1" :!type "EObjectTypeQuery Enum")))
  (set `self.HMD_Origin` (`KismetMathLibrary.InverseTransformLocation` (`SceneComponent.K2_GetComponentToWorld` (`self.CapsuleComponent`)) (`.Location` (`GameplayStatics.BreakHitResult` _outhit)))))

(fn `Movement`
  (params (Value :type "Float (double-precision)"))
  ;[1 1 1] Forward and Backward Movement
  (`self.AddMovementInput` (`SceneComponent.GetForwardVector` (`self.Camera`)) Value))

(fn `Rotation`
  (params (value :type "Float (double-precision)"))
  (bind (_returnvalue_roll _returnvalue_pitch _returnvalue_yaw) (`KismetMathLibrary.BreakRotator` (`self.K2_GetActorRotation`)))
  (bind (_returnvalue_roll_2 _returnvalue_pitch_2 _returnvalue_yaw_2) (`KismetMathLibrary.BreakRotator` (`self.K2_GetActorRotation`)))
  (bind _snap_rotation_degrees (`self.Snap Rotation Degrees`))
  (bind _returnvalue (> (`KismetMathLibrary.Abs` value) (`self.Turn Deadzone`)))
  ;[1 1 1] Rotation
  (if _returnvalue
    (`/Engine/EditorBlueprintResources/StandardMacros.DoOnce` false :!label _label
      (:`Completed`
        ;;[0.1771 0.1771 0.1771] Check for Snap or Continuous Rotation
        (if (`self.bSmoothRotation`)
          (if true
            ;;[0.1562 0.1562 0.1562] Continuous Rotation
            (`self.K2_SetActorRotation` (`KismetMathLibrary.MakeRotator` 0.0 0.0 (+ _returnvalue_yaw (* value (`self.Smooth Rotation Speed`))))))
          (elif _returnvalue
            ;;[0.1562 0.1562 0.1562] Snap Rotation
            (if (> value 0.4)
              (set `self.Rotation Angle` _snap_rotation_degrees)
              (else
                (set `self.Rotation Angle` (* -1.0 _snap_rotation_degrees))))
            (`/Engine/EditorBlueprintResources/StandardMacros.DoOnce` false :!label _label_2
              (:`Completed`
                (`|ExecutionSequence`
                  (:`then_0`
                    (`self.K2_SetActorRotation` (`KismetMathLibrary.MakeRotator` 0.0 0.0 (+ _returnvalue_yaw_2 (`self.Rotation Angle`)))))
                  (:`then_1`
                    (goto _label_2 :!via `Reset`)))))))))
    (else
      (goto _label :!via `Reset`))))

(fn `Strafe`
  (params (value :type "Float (double-precision)"))
  ;[1 1 1] Strafe Movement Input
  (`self.AddMovementInput` (`SceneComponent.GetRightVector` (`self.Camera`)) value))

(fn `UserConstructionScript`)