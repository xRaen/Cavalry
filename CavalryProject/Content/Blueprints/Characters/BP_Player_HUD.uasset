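; VR player character that spawns and attaches two motion controllers and horseman-specific gear, setting floor tracking for Oculus and Windows Mixed Reality headsets.
; Movement and strafe functions follow camera direction, while snap or smooth turning shares a deadzone-reset DoOnce, stepping once per stick deflection.
; Damage drains shields, then counts health hits with a three-second immunity window until Death, which only prints a message.
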(event `self.ReceiveBeginPlay`
  (bind _returnvalue (`KismetMathLibrary.MakeTransform` (0.0 0.0 0.0)))
  (`|ExecutionSequence`
    (:`then_0`
      ;[0 0 0] Setup Player Height for Each HMD [Oculus, Odyssey, SteamVR]
      (switch `name` (`HeadMountedDisplayFunctionLibrary.GetHMDDeviceName`)
        (:`Oculus HMD`
          _)
        (:`Windows Mixed Reality`
          _))
      (`HeadMountedDisplayFunctionLibrary.SetTrackingOrigin` "Floor"))
    (:`then_1`
      (`|ExecutionSequence`
        (:`then_0`
          ;[0 0 0] Motion Controller Spawn and Attach
          (bind _returnvalue_2 (`|SpawnActorFromClass` "/Game/VirtualRealityBP/Blueprints/BP_MotionController.BP_MotionController_C" _returnvalue "AlwaysSpawn" "OverrideRootScale" self "Left" null))
          (set `self.Left Controller` _returnvalue_2)
          (`self.K2_AttachToComponent` _returnvalue_2 (`self.CapsuleComponent`) "None" "SnapToTarget" "SnapToTarget" "KeepWorld" false))
        (:`then_1`
          (bind _returnvalue_3 (`|SpawnActorFromClass` "/Game/VirtualRealityBP/Blueprints/BP_MotionController.BP_MotionController_C" _returnvalue "AlwaysSpawn" "OverrideRootScale" self "Right" null))
          (set `self.Right Controller` _returnvalue_3)
          (`self.K2_AttachToComponent` _returnvalue_3 (`self.CapsuleComponent`) "None" "SnapToTarget" "SnapToTarget" "KeepWorld" false))
        (:`then_2`
          ;[0 0 0] Gear Spawning (default horseman is War)
          (bind _returnvalue_4 (`|SpawnActorFromClass` "/Game/Blueprints/Characters/Gear/BP_PlayerGear.BP_PlayerGear_C" (`KismetMathLibrary.MakeTransform` (0.0 0.0 0.0)) "AlwaysSpawn" "OverrideRootScale" self (`self.Horseman to Spawn For`) null))
          (bind _output_get (set `self.PlayerGear` _returnvalue_4))
          (`self.K2_AttachToComponent` _output_get (`self.GearLoction`) "None" "SnapToTarget" "SnapToTarget" "SnapToTarget" false))))))

(event `/Game/Blueprints/Interfaces/BPI_TakeDamage.TakeDamage`
  (params (DamageAmount :type Integer))
  (bind _currentshields (`self.currentShields`))
  ;[0 0 0] Taking Damage
  (if (not (`self.recentlyHit`))
    (set `self.currentShields` (- _currentshields DamageAmount))
    (if (<= _currentshields 0)
      (set `self.currentShields` 0)
      (`/Engine/EditorBlueprintResources/StandardMacros.IncrementInt` (`self.healthHits`)
        (:`  `
          (set `self.recentlyHit` true)
          (`KismetSystemLibrary.K2_SetTimerDelegate` (delegate `ResetHitTimer`) 3.0)
          ;[0 0 0] Should player be dead?
          (if (>= (`self.healthHits`) (`self.maxHealthHits`))
            (`self.Death`)))))))

(event `ResetHitTimer`
  ;[0 0 0] Taking Damage
  (set `self.recentlyHit` false))

(event `Death`
  ;[0 0 0] Player Death
  (`KismetSystemLibrary.PrintString` "You are dead :)"))

(fn `Movement`
  (params (Value :type "Float (double-precision)"))
  ;[0 0 0] Forward and Backward Movement
  (`self.AddMovementInput` (`SceneComponent.GetForwardVector` (`self.Camera`)) Value))

(fn `Rotation`
  (params (value :type "Float (double-precision)"))
  (bind (_returnvalue_roll _returnvalue_pitch _returnvalue_yaw) (`KismetMathLibrary.BreakRotator` (`self.K2_GetActorRotation`)))
  (bind (_returnvalue_roll_2 _returnvalue_pitch_2 _returnvalue_yaw_2) (`KismetMathLibrary.BreakRotator` (`self.K2_GetActorRotation`)))
  (bind _snap_rotation_degrees (`self.Snap Rotation Degrees`))
  (bind _returnvalue (> (`KismetMathLibrary.Abs` value) (`self.Turn Deadzone`)))
  ;[0 0 0] Rotation
  (if _returnvalue
    (`/Engine/EditorBlueprintResources/StandardMacros.DoOnce` false :!label _label
      (:`Completed`
        ;;[0.1771 0.1771 0.1771] Check for Snap or Continuous Rotation
        (if (`self.bSmoothRotation`)
          (if true
            ;;[0.1562 0.1562 0.1562] Continuous Rotation
            (`self.K2_SetActorRotation` (`KismetMathLibrary.MakeRotator` 0.0 0.0 (+ _returnvalue_yaw (* value (`self.Smooth Rotation Speed`))))))
          (elif _returnvalue
            ;;[0.1562 0.1562 0.1562] Snap Rotation
            (if (> value 0.2)
              (set `self.Rotation Angle` _snap_rotation_degrees)
              (else
                (set `self.Rotation Angle` (* -1.0 _snap_rotation_degrees))))
            (`/Engine/EditorBlueprintResources/StandardMacros.DoOnce` false :!label _label_2
              (:`Completed`
                (`|ExecutionSequence`
                  (:`then_0`
                    (`self.K2_SetActorRotation` (`KismetMathLibrary.MakeRotator` 0.0 0.0 (+ _returnvalue_yaw_2 (`self.Rotation Angle`)))))
                  (:`then_1`
                    (goto _label_2 :!via `Reset`)))))))))
    (else
      (goto _label :!via `Reset`))))

(fn `Strafe`
  (params (value :type "Float (double-precision)"))
  ;[0 0 0] Strafe Movement Input
  (`self.AddMovementInput` (`SceneComponent.GetRightVector` (`self.Camera`)) value))

(fn `UserConstructionScript`)