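; GrabbableObjectSocket is a grab component that snaps an object onto a named socket and later releases it.
; Grab, gated by ComponentActive, stores the mesh and root actor, disables physics, then attaches the actor's root, snapping location and rotation while keeping world scale.
; Release uses the stored references to re-enable physics and detach the actor, keeping its world transform, without checking ComponentActive.
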(event `Grab`
  (params (StaticMeshComponent :type "MeshComponent Object Reference") (RootActor :type "Actor Object Reference") (AttachTo :type "SceneComponent Object Reference") (SocketName :type Name))
  (if (`self.ComponentActive`)
    (bind _output_get (set `self.StaticMeshComponent` StaticMeshComponent))
    (bind _output_get_2 (set `self.RootActor` RootActor))
    (`PrimitiveComponent.SetSimulatePhysics` _output_get false)
    (`SceneComponent.K2_AttachToComponent` (`Actor.K2_GetRootComponent` _output_get_2) AttachTo SocketName "SnapToTarget" "SnapToTarget" "KeepWorld" false)))

(event `Release`
  (`PrimitiveComponent.SetSimulatePhysics` (`self.StaticMeshComponent`) true)
  (`Actor.K2_DetachFromActor` (`self.RootActor`) "KeepWorld" "KeepWorld" "KeepWorld"))