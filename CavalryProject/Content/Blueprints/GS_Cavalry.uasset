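; GS_Cavalry is the game state that tracks mission objectives and team wipes.
; It counts hostages and player controllers at BeginPlay, then broadcasts hostage objective completion once all are rescued.
; Rescuing all hostages and stopping the server download completes phase one, triggering the security lockdown after a short delay.
; All players dying returns to MainMenu after a delay, while the lockdown-lifted and missile-stopped events are empty stubs.
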(event `self.ReceiveBeginPlay`
  (bind _outactors (`GameplayStatics.GetAllActorsOfClass` "/Game/Blueprints/LF-19/BP_HostageTest.BP_HostageTest_C"))
  (set `self.HostageArray` _outactors)
  (bind _outactors_2 (`GameplayStatics.GetAllActorsOfClass` "/Game/Blueprints/Characters/BP_CavalryController.BP_CavalryController_C"))
  (set `self.PlayerCount` (`KismetArrayLibrary.Array_Length` _outactors_2))
  (set `self.DeadPlayerCount` 0))

(event `/Game/Blueprints/Interfaces/BPI_GameStateCommunication.HostageRescued`
  (bind _result (`/Engine/EditorBlueprintResources/StandardMacros.IncrementInt` (`self.HostageRescueCount`))
    (:`  `
      (if (>= _result (`KismetArrayLibrary.Array_Length` (`self.HostageArray`)))
        (set `self.HostagesRescued` true)
        (`self.Phase1CompletionCheck`)
        (`self.HostageObjectiveComplete`)))))

(event `/Game/Blueprints/Interfaces/BPI_GameStateCommunication.ServerDownloadStopped`
  (set `self.ServerDonwloadStopped` true)
  (`self.Phase1CompletionCheck`))

(event `Phase1CompletionCheck`
  (if (and (`self.HostagesRescued`) (`self.ServerDonwloadStopped`))
    (`KismetSystemLibrary.Delay` 2.0)
    (`self.SecurityLockdownStart`)))

(event `/Game/Blueprints/Interfaces/BPI_GameStateCommunication.SecurityLockdownLifted`)

(event `/Game/Blueprints/Interfaces/BPI_GameStateCommunication.MissileLaunchStopped`)

(event `AllPlayersDeadCheck`
  (bind _deadplayercount (`self.DeadPlayerCount`))
  (`/Engine/EditorBlueprintResources/StandardMacros.IncrementInt` _deadplayercount
    (:`  `
      (if (>= _deadplayercount (`self.PlayerCount`))
        (`KismetSystemLibrary.Delay` 5.0)
        (`GameplayStatics.OpenLevel` "MainMenu")))))

(fn `UserConstructionScript`)