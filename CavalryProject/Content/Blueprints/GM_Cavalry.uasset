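; GM_Cavalry is the Cavalry game mode, which spawns and possesses the player's pawn when play begins.
; On BeginPlay it reads the PlayerToSpawn class from BP_Cavalry_GameInstance, spawns it at the first PlayerStart found and has player controller 0 possess it.
; Mission events for rescued hostages, a stopped server upload and a stopped missile launch are declared but empty.
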(event `self.ReceiveBeginPlay`
  (bind _asbp_cavalry_game_instance (cast `/Game/HUD/Main_Menu/BP_Cavalry_GameInstance` (`GameplayStatics.GetGameInstance`)))
  (bind _outactors (`GameplayStatics.GetAllActorsOfClass` "/Script/Engine.PlayerStart"))
  (bind _output (`|GetArrayItem` _outactors))
  (if (`KismetSystemLibrary.IsValid` _output)
    (bind _returnvalue (`|SpawnActorFromClass` (`/Game/HUD/Main_Menu/BP_Cavalry_GameInstance.PlayerToSpawn` _asbp_cavalry_game_instance) (`self.GetTransform` _output) "Undefined" "OverrideRootScale" null null))
    (`Controller.Possess` (`GameplayStatics.GetPlayerController` 0) _returnvalue)))

(event `/Game/Blueprints/Interfaces/BPI_GameModeCommunication.HostagesRescued`)

(event `/Game/Blueprints/Interfaces/BPI_GameModeCommunication.ServerUploadStopped`)

(event `/Game/Blueprints/Interfaces/BPI_GameModeCommunication.MissileLaunchStopped`)

(fn `UserConstructionScript`)