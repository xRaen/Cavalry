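; Base VR firearm with two-handed grabbing, firing, reloading and magnetic holstering.
; The first hand holds the gun; a second either racks the slider or steers aim, whichever collider is nearer, via timelines.
; Fire modes drive short line-trace shots that damage enemies, while load type selects magazine or shell handling and slider overlaps re-arm firing.
; On release, it snaps to the closest free, compatible overlapping magnet mount.
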(event `SecondHandRelease`
  (bind _second_hand_mesh (`self.Second Hand Mesh`))
  ;[0 0 0] Comment
  (`SceneComponent.K2_DetachFromComponent` _second_hand_mesh "KeepWorld" "KeepWorld" "KeepWorld" true)
  (`SceneComponent.K2_AttachToComponent` _second_hand_mesh (`/Game/VirtualRealityBP/Blueprints/BP_MotionController.MotionController` (`self.Second Hand Motion Controller`)) "None" "SnapToTarget" "SnapToTarget" "KeepWorld" true)
  (`SceneComponent.K2_SetRelativeRotation` _second_hand_mesh (struct :`Roll` -90.0) false false)
  (`SceneComponent.K2_SetRelativeLocation` _second_hand_mesh (-15.0 0.0 0.0) false false)
  (if (`|EnumEquality` (`self.dominantHand`) "Left")
    ;;[0.1094 0.1094 0.1094] Left Hand Dominant
    (`SceneComponent.K2_SetRelativeRotation` :`self` (`self.Firearm_SM`))
    (else
      ;;[0.1094 0.1094 0.1094] Right Hand Dominant
      (`SceneComponent.K2_SetRelativeRotation` (`self.Firearm_SM`) (struct :`Roll` 180.0) false false))))

(event `SliderRevertPosition`
  ;[0 0 0] Slider Reset
  (`KismetSystemLibrary.MoveComponentTo` (`self.Slider_SM`) (0.0 0.0 0.0) (struct) false false 0.1)
  (set `self.SecondHandGrabbed` false))

(event `self.Slider_Stopper.OnComponentBeginOverlap`
  (params (OverlappedComponent :type "PrimitiveComponent Object Reference") (OtherActor :type "Actor Object Reference") (OtherComp :type "PrimitiveComponent Object Reference") (OtherBodyIndex :type Integer) (bFromSweep :type Boolean) (SweepResult :type "HitResult Structure (by ref)"))
  ;[0 0 0] Slider Reset
  (if (== OtherComp (`self.Slider_Collider`))
    (set `self.CockedBack` true)))

(event `self.Slider_ForwardPosition.OnComponentBeginOverlap`
  (params (OverlappedComponent :type "PrimitiveComponent Object Reference") (OtherActor :type "Actor Object Reference") (OtherComp :type "PrimitiveComponent Object Reference") (OtherBodyIndex :type Integer) (bFromSweep :type Boolean) (SweepResult :type "HitResult Structure (by ref)"))
  ;[0 0 0] Slider Reset
  (if (== OtherComp (`self.Slider_Collider`))
    (if (`self.CockedBack`)
      (set `self.CockedBack` false)
      (set `self.canFire` true))))

(event `/Game/Blueprints/Interfaces/BPI_GrabbableObj.Grab`
  (params (HandSocket :type Name) (AttachToMe :type "SceneComponent Object Reference") (Actor :type "Actor Object Reference"))
  (bind _x_last_position_x (`KismetMathLibrary.BreakVector` (`self.X_Last_Position`)))
  (bind _slider_sm (`self.Slider_SM`))
  (bind _x_last_position_x_2 (`KismetMathLibrary.BreakVector` (`self.X_Last_Position`)))
  (bind _returnvalue_location (`KismetMathLibrary.BreakTransform` (`SceneComponent.K2_GetComponentToWorld` (`self.Firearm_SM`))))
  (bind _relativelocation_x (`KismetMathLibrary.BreakVector` (`SceneComponent.RelativeLocation` _slider_sm)))
  (bind _relativelocation_x_2 (`KismetMathLibrary.BreakVector` (`SceneComponent.RelativeLocation` _slider_sm)))
  (bind _returnvalue_x (`KismetMathLibrary.BreakVector` (`KismetMathLibrary.InverseTransformLocation` (`SceneComponent.K2_GetComponentToWorld` (`self.Firearm_SM`)) (`SceneComponent.K2_GetComponentLocation` (`/Game/VirtualRealityBP/Blueprints/BP_MotionController.MotionController` (`self.Second Hand Motion Controller`))))))
  (bind _returnvalue_x_2 (`KismetMathLibrary.BreakVector` (`KismetMathLibrary.InverseTransformLocation` (`SceneComponent.K2_GetComponentToWorld` (`self.Firearm_SM`)) (`SceneComponent.K2_GetComponentLocation` (`/Game/VirtualRealityBP/Blueprints/BP_MotionController.MotionController` (`self.Second Hand Motion Controller`))))))
  ;[0 0 0] Grabbing
  (if (`self.FirstHandGrabbed`)
    ;;[0.1329 0.1329 0.1329] Which Collider is closer?
    (bind _asbp_motion_controller (cast `/Game/VirtualRealityBP/Blueprints/BP_MotionController` Actor))
    (bind _returnvalue (`SceneComponent.K2_GetComponentLocation` (`/Game/VirtualRealityBP/Blueprints/BP_MotionController.MotionController` _asbp_motion_controller)))
    (if (< (`KismetMathLibrary.VSize` (- _returnvalue (`SceneComponent.K2_GetComponentLocation` (`self.Slider_Collider`)))) (`KismetMathLibrary.VSize` (- _returnvalue (`SceneComponent.K2_GetComponentLocation` (`self.SecondHand_Collider`)))))
      ;;[0.1333 0.1333 0.1333] Slider Grab
      (set `self.SecondHandGrabbed` true)
      (bind _output_get (set `self.Second Hand Motion Controller` _asbp_motion_controller))
      (set `self.Second Hand Mesh` AttachToMe)
      (set `self.X_Last_Position` (`KismetMathLibrary.MakeVector` _returnvalue_x_2))
      (set `/Game/VirtualRealityBP/Blueprints/BP_MotionController.GripState` "NewEnumerator3" _output_get)
      (`Timeline|SliderMovementTimeline` :!via `PlayFromStart` :!label _label
        (:`Update`
          (if (`|EnumInequality` (`/Game/VirtualRealityBP/Blueprints/BP_MotionController.GripState` (`self.Second Hand Motion Controller`)) "NewEnumerator0")
            (if (`self.SecondHandGrabbed`)
              (bind _output_get_2 (set `self.X_Delta` (- _returnvalue_x _x_last_position_x)))
              (set `self.X_Last_Position` (`KismetMathLibrary.MakeVector` (+ _output_get_2 _x_last_position_x_2)))
              (`SceneComponent.K2_AddRelativeLocation` _slider_sm (`KismetMathLibrary.MakeVector` _output_get_2) true true)
              (if (> _relativelocation_x_2 (`self.SliderXMax`))
                (`SceneComponent.K2_SetRelativeLocation` _slider_sm (0.0 0.0 0.0) false false)
                (elif (< _relativelocation_x (`self.SliderXMin`))
                  (`SceneComponent.K2_SetRelativeLocation` _slider_sm (-10.0 0.0 0.0) false false)))
              (else
                (`self.SliderRevertPosition` :!label _label_2)
                (goto _label :!via `Stop`)))
            (else
              (goto _label_2)))))
      (else
        ;;[0.1329 0.1329 0.1329] Second Hand Guide
        (set `self.SecondHandGrabbed` true)
        (`SceneComponent.K2_AttachToComponent` AttachToMe (`self.Firearm_SM`) "Second_Hand_Socket" "SnapToTarget" "SnapToTarget" "KeepWorld" true)
        (bind _output_get_3 (set `self.Second Hand Motion Controller` _asbp_motion_controller))
        (set `/Game/VirtualRealityBP/Blueprints/BP_MotionController.GripState` "NewEnumerator3" _output_get_3)
        (set `self.Second Hand Mesh` AttachToMe)
        (`KismetSystemLibrary.Delay` 0.1)
        (`Timeline|Timeline_0` :!label _label_3
          (:`Update`
            (if (`|EnumInequality` (`/Game/VirtualRealityBP/Blueprints/BP_MotionController.GripState` (`self.Second Hand Motion Controller`)) "NewEnumerator0")
              (if (`self.SecondHandGrabbed`)
                (`SceneComponent.K2_SetWorldRotation` (`self.Firearm_SM`) (`KismetMathLibrary.FindLookAtRotation` _returnvalue_location (`SceneComponent.K2_GetComponentLocation` (`/Game/VirtualRealityBP/Blueprints/BP_MotionController.MotionController` (`self.Second Hand Motion Controller`)))) false false)
                (else
                  (`self.SecondHandRelease` :!label _label_4)
                  (goto _label_3 :!via `Stop`)))
              (else
                (goto _label_4)))))))
    (else
      ;;[0.1771 0.1771 0.1771] First Hand Grabbed
      (if (`self.OnMagnetMount`)
        (set `/Game/Blueprints/Tools/BP_MagneticPlacement.Occupied` false (`self.MagnetMount`))
        (set `self.OnMagnetMount` false)
        (set `self.ClosestMount` null))
      (`/Game/Blueprints/GrabbableObjectSocket.Grab` (`self.GrabbableObjectSocket`) (`self.Firearm_SM`) self HandSocket AttachToMe)
      (set `self.FirstHandGrabbed` true)
      (set `self.SecondHandGrabbed` false)
      (set `self.First Hand` AttachToMe)
      (bind _asbp_motion_controller_2 (cast `/Game/VirtualRealityBP/Blueprints/BP_MotionController` Actor))
      (set `self.dominantHand` (`/Game/VirtualRealityBP/Blueprints/BP_MotionController.Hand` _asbp_motion_controller_2))
      (set `/Game/VirtualRealityBP/Blueprints/BP_MotionController.GripState` "NewEnumerator2" _asbp_motion_controller_2))))

(event `/Game/Blueprints/Interfaces/BPI_GrabbableObj.Release`
  ;[0 0 0] Releasing
  (`/Game/Blueprints/GrabbableObjectSocket.Release` (`self.GrabbableObjectSocket`))
  (set `self.FirstHandGrabbed` false)
  (if (`self.SecondHandGrabbed`)
    (set `self.SecondHandGrabbed` false)
    (set `/Game/VirtualRealityBP/Blueprints/BP_MotionController.GripState` "NewEnumerator0" (`self.Second Hand Motion Controller`))
    (set `self.isFiring` false))
  (if (not (== (`KismetArrayLibrary.Array_Length` (`self.OverlappingMagnets`)) 0))
    (`self.Magnetize` null)))

(event `/Game/Blueprints/Interfaces/BPI_WeaponControls.ShootRelease`
  ;[0 0 0] Player Input
  ;;[0.1413 0.1413 0.1413] Comment
  (set `self.isFiring` false))

(event `/Game/Blueprints/Interfaces/BPI_WeaponControls.Shoot`
  (params (Hand :type "/Game/Blueprints/Enums/E_Hands Enum" :default "NewEnumerator0"))
  ;[0 0 0] Player Input
  ;;[0.07819 0.07819 0.07819] Left Primary Trigger
  (set `self.isFiring` true)
  (switch `/Game/Blueprints/Enums/E_FireMode` (`self.currentFireMode`)
    (:`NewEnumerator0`
      (`self.Fire`)
      (`KismetSystemLibrary.Delay` (`self.firerate`))
      (set `self.isFiring` false))
    (:`NewEnumerator2`
      (`KismetSystemLibrary.K2_SetTimerDelegate` (delegate `Fire`) (`self.firerate`) (`self.isFiring`)))))

(event `/Game/Blueprints/Interfaces/BPI_WeaponControls.ReleaseMagazine`
  ;[0 0 0] Player Input
  ;;[0.07819 0.07819 0.07819] Right Primary Button
  (if (`self.FirstHandGrabbed`)
    (`self.Release Magazine`)))

(event `/Game/Blueprints/Interfaces/BPI_WeaponControls.ChangeFiremode`
  ;[0 0 0] Player Input
  ;;[0.07819 0.07819 0.07819] Right Secondary Button
  (if (`self.FirstHandGrabbed`)
    (`self.Change Fire Mode`)))

(event `Fire`
  (bind _firelocation (`self.FireLocation`))
  (bind _returnvalue (`SceneComponent.K2_GetComponentLocation` _firelocation))
  ;[0 0 0] Firing
  (if (`self.canFire`)
    (if (`self.isLoaded`)
      (if (> (`self.currentAmmo`) 0)
        (switch `/Game/Blueprints/Enums/E_LoadType` (`self.loadType`)
          (:`NewEnumerator0`
            _)
          (:`NewEnumerator2`
            _)
          (:`NewEnumerator3`
            _)
          (:`NewEnumerator4`
            _)
          (:`NewEnumerator1`
            (set `self.canFire` false)))
        (`/Engine/EditorBlueprintResources/StandardMacros.DecrementInt` (`self.currentAmmo`)
          (:`  `
            (`|SpawnActorFromClass` "/Game/Blueprints/Weapons/BP_BulletBase.BP_BulletBase_C" (`SceneComponent.K2_GetComponentToWorld` (`self.ShellEjectionPoint`)) "AdjustIfPossibleButAlwaysSpawn" "OverrideRootScale" null null)
            (bind _outhit (`KismetSystemLibrary.LineTraceSingleForObjects` :`Start` _returnvalue :`End` (+ _returnvalue (* (`KismetMathLibrary.GetForwardVector` (`SceneComponent.K2_GetComponentRotation` _firelocation)) 200)) :`ObjectTypes` (`|MakeArray` "ObjectTypeQuery7" "ObjectTypeQuery1" :!type "EObjectTypeQuery Enum") :`DrawDebugType` "Persistent"))
            (`NiagaraFunctionLibrary.SpawnSystemAttached` "/Game/VisualEffects/Niagara/NS_muzzle_flash.NS_muzzle_flash" (`self.Niagara`) "None" (0.0 0.0 0.0) (struct) "KeepRelativeOffset")
            (`KismetSystemLibrary.PrintString` "FIRING")
            (switch `ECollisionChannel` (`PrimitiveComponent.GetCollisionObjectType` (`.HitComponent` (`GameplayStatics.BreakHitResult` _outhit)))
              (:`ECC_WorldStatic`
                (`KismetSystemLibrary.PrintString` "Gun hit Static Geo"))
              (:`ECC_GameTraceChannel1`
                (`KismetSystemLibrary.PrintString` "Gun hit Enemy")
                (message `/Game/Blueprints/Interfaces/BPI_TakeDamage.TakeDamage` (`.HitComponent` (`GameplayStatics.BreakHitResult` _outhit)) (`self.damageAmount`)))
              (:`ECC_GameTraceChannel4`
                (`KismetSystemLibrary.PrintString` "Gun hit Shield")))))
        (else
          (set `self.canFire` false))))))

(event `Change Fire Mode`
  ;[0 0 0] Changing Fire Mode
  (if (`self.canAutomatic`)
    (if (not (`self.isFiring`))
      (switch `/Game/Blueprints/Enums/E_FireMode` (`self.currentFireMode`)
        (:`NewEnumerator0`
          (set `self.currentFireMode` "NewEnumerator2"))
        (:`NewEnumerator2`
          (set `self.currentFireMode` "NewEnumerator0"))))))

(event `Reload`
  (params (BP_AmmoBase :type "/Game/Blueprints/Weapons/BP_AmmoBase Object Reference") (`Magazine Base` :type Integer))
  ;[0 0 0] Reloading
  (if (`|EnumEquality` (`/Game/Blueprints/Weapons/BP_AmmoBase.AmmoType` BP_AmmoBase) (`self.loadType`))
    (if (not (`self.isFiring`))
      (switch `/Game/Blueprints/Enums/E_LoadType` (`self.loadType`)
        (:`NewEnumerator0`
          ;;[0.07819 0.07819 0.07819] Magazine
          (set `self.magazineObj` BP_AmmoBase :!label _label_5)
          (set `self.currentAmmo` `Magazine Base`)
          (set `self.isLoaded` true :!label _label_6))
        (:`NewEnumerator2`
          (goto _label_5))
        (:`NewEnumerator3`
          (goto _label_5))
        (:`NewEnumerator4`
          (goto _label_5))
        (:`NewEnumerator1`
          ;;[0.07819 0.07819 0.07819] Shells
          (if (< (`self.currentAmmo`) 6)
            (`/Engine/EditorBlueprintResources/StandardMacros.IncrementInt` (`self.currentAmmo`)
              (:`  `
                (`self.K2_DestroyActor` BP_AmmoBase)
                (goto _label_6)))))))))

(event `Release Magazine`
  (bind _magazineobj (`self.magazineObj`))
  ;[0 0 0] Ammo Ejection
  (if (not (`self.isFiring`))
    (switch `/Game/Blueprints/Enums/E_LoadType` (`self.loadType`)
      (:`NewEnumerator0`
        ;;[0.07819 0.07819 0.07819] Magazine
        (set `self.currentAmmo` 0 :!label _label_7)
        (`self.K2_DetachFromActor` _magazineobj "KeepWorld" "KeepWorld" "KeepWorld")
        (`PrimitiveComponent.SetSimulatePhysics` (`/Game/Blueprints/Weapons/BP_AmmoBase.Ammo_SM` _magazineobj) true)
        (set `self.isLoaded` false :!label _label_8)
        (`KismetSystemLibrary.PrintString` "BP_Firearm_Base: magazine has been dropped" true true (struct :`R` 0.042945 :`B` 1.0 :`A` 1.0) 15.0))
      (:`NewEnumerator2`
        (goto _label_7))
      (:`NewEnumerator3`
        (goto _label_7))
      (:`NewEnumerator4`
        (goto _label_7))
      (:`NewEnumerator1`
        ;;[0.07819 0.07819 0.07819] Shells
        (if (< (`self.currentAmmo`) 1)
          (goto _label_8))))))

(event `self.Magnetize`
  (params (Magnet :type "Actor Object Reference"))
  (bind _closestmount (`self.ClosestMount`))
  (bind _firearm_sm (`self.Firearm_SM`))
  (bind _returnvalue (`SceneComponent.K2_GetComponentLocation` (`self.MagnetCollision`)))
  ;[0 0 0] Magnetic
  (set `self.ClosestMount` null)
  (if (not (`self.FirstHandGrabbed`))
    (for _array_element (`self.OverlappingMagnets`)
      (if (`/Game/Blueprints/Tools/BP_MagneticPlacement.Occupied` _array_element)
        _
        (elif (or (`|EnumEquality` (`self.WeaponObjectType`) (`/Game/Blueprints/Tools/BP_MagneticPlacement.Object Type` _array_element)) (`|EnumEquality` (`/Game/Blueprints/Tools/BP_MagneticPlacement.Object Type` _array_element) "NewEnumerator0"))
          (if (`KismetSystemLibrary.IsValid` (`self.ClosestMount`))
            (if (< (`KismetMathLibrary.VSize` (- _returnvalue (`SceneComponent.K2_GetComponentLocation` (`Actor.RootComponent` _array_element)))) (`KismetMathLibrary.VSize` (- _returnvalue (`SceneComponent.K2_GetComponentLocation` (`Actor.RootComponent` (`self.ClosestMount`))))))
              (set `self.ClosestMount` _array_element))
            (else
              (set `self.ClosestMount` _array_element))))))
    (if (`KismetSystemLibrary.IsValid` (`self.ClosestMount`))
      (`PrimitiveComponent.SetSimulatePhysics` _firearm_sm false)
      (`SceneComponent.K2_AttachToComponent` _firearm_sm (`Actor.RootComponent` _closestmount) "None" "SnapToTarget" "SnapToTarget" "KeepWorld" false)
      (set `self.OnMagnetMount` true)
      (bind _output_get (set `self.MagnetMount` _closestmount))
      (set `/Game/Blueprints/Tools/BP_MagneticPlacement.Occupied` true _output_get))))

(event `self.MagnetCollision.OnComponentBeginOverlap`
  (params (OverlappedComponent :type "PrimitiveComponent Object Reference") (OtherActor :type "Actor Object Reference") (OtherComp :type "PrimitiveComponent Object Reference") (OtherBodyIndex :type Integer) (bFromSweep :type Boolean) (SweepResult :type "HitResult Structure (by ref)"))
  ;[0 0 0] Magnetic
  (bind _asbp_magnetic_placement (cast `/Game/Blueprints/Tools/BP_MagneticPlacement` OtherActor))
  (`KismetArrayLibrary.Array_Add` (`self.OverlappingMagnets`) _asbp_magnetic_placement))

(event `self.MagnetCollision.OnComponentEndOverlap`
  (params (OverlappedComponent :type "PrimitiveComponent Object Reference") (OtherActor :type "Actor Object Reference") (OtherComp :type "PrimitiveComponent Object Reference") (OtherBodyIndex :type Integer))
  ;[0 0 0] Magnetic
  (bind _asbp_magnetic_placement (cast `/Game/Blueprints/Tools/BP_MagneticPlacement` OtherActor))
  (`KismetArrayLibrary.Array_RemoveItem` (`self.OverlappingMagnets`) _asbp_magnetic_placement))

(fn `UserConstructionScript`)