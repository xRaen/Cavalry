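; Prototype firearm actor with a slide that follows an overlapping component, treated as the second hand, along the gun's X axis.
; Any overlap on the slider collider stores that component and prints a debug message.
; Tick applies its movement in firearm local space to the slide with sweep, capping X at zero.
; When the slider collider hits the stopper, tracking ends and MoveComponentTo quickly snaps the slide to its default target.
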(event `self.Slider_Collider.OnComponentBeginOverlap`
  (params (OverlappedComponent :type "PrimitiveComponent Object Reference") (OtherActor :type "Actor Object Reference") (OtherComp :type "PrimitiveComponent Object Reference") (OtherBodyIndex :type Integer) (bFromSweep :type Boolean) (SweepResult :type "HitResult Structure (by ref)"))
  (bind _returnvalue_x (`KismetMathLibrary.BreakVector` (`KismetMathLibrary.InverseTransformLocation` (`SceneComponent.K2_GetComponentToWorld` (`self.Firearm_SM`)) (`SceneComponent.K2_GetComponentLocation` (`self.Second Hand`)))))
  (`KismetSystemLibrary.PrintString` "Hello")
  (set `self.Second Hand Object` null)
  (set `self.Second Hand` OtherComp)
  (set `self.X_Last_Position` (`KismetMathLibrary.MakeVector` _returnvalue_x))
  (set `self.Condition` true))

(event `self.ReceiveTick`
  (params (DeltaSeconds :type "Float (single-precision)"))
  (bind _x_last_position_x (`KismetMathLibrary.BreakVector` (`self.X_Last_Position`)))
  (bind _slider_sm (`self.Slider_SM`))
  (bind _x_last_position_x_2 (`KismetMathLibrary.BreakVector` (`self.X_Last_Position`)))
  (bind _relativelocation_x (`KismetMathLibrary.BreakVector` (`SceneComponent.RelativeLocation` _slider_sm)))
  (bind _returnvalue_x (`KismetMathLibrary.BreakVector` (`KismetMathLibrary.InverseTransformLocation` (`SceneComponent.K2_GetComponentToWorld` (`self.Firearm_SM`)) (`SceneComponent.K2_GetComponentLocation` (`self.Second Hand`)))))
  (if (`self.Condition`)
    (bind _output_get (set `self.X_Delta` (- _returnvalue_x _x_last_position_x)))
    (set `self.X_Last_Position` (`KismetMathLibrary.MakeVector` (+ _output_get _x_last_position_x_2)))
    (`SceneComponent.K2_AddRelativeLocation` _slider_sm (`KismetMathLibrary.MakeVector` _output_get) true true)
    (if (> _relativelocation_x 0.0)
      (`SceneComponent.K2_SetRelativeLocation` _slider_sm (0.0 0.0 0.0) false false))))

(event `self.Slider_Stopper.OnComponentBeginOverlap`
  (params (OverlappedComponent :type "PrimitiveComponent Object Reference") (OtherActor :type "Actor Object Reference") (OtherComp :type "PrimitiveComponent Object Reference") (OtherBodyIndex :type Integer) (bFromSweep :type Boolean) (SweepResult :type "HitResult Structure (by ref)"))
  (if (== OtherComp (`self.Slider_Collider`))
    (set `self.Condition` false)
    (`KismetSystemLibrary.MoveComponentTo` (`self.Slider_SM`) (0.0 0.0 0.0) (struct) false false 0.01)))

(fn `UserConstructionScript`)