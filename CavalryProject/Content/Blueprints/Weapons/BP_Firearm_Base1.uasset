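; Base VR firearm actor that is grabbed by motion controllers and supports single or automatic fire.
; Dominant-hand trigger input calls Fire directly or by timer, spending ammo on a short forward line trace that damages enemies.
; An ammo port overlap loads magazines or shells by load type, and a button ejects magazines or clears spent shells.
; A timeline makes the slide follow the second hand's X position until its grip state changes.
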(event `Slider Release`
  ;[0 0 0] Slider Release & Snap
  (bind _asbp_motion_controller (cast `/Game/VirtualRealityBP/Blueprints/BP_MotionController` (`self.Second Hand`)))
  (set `/Game/VirtualRealityBP/Blueprints/BP_MotionController.GripState` "NewEnumerator0" _asbp_motion_controller))

(event `self.Slider_Collider.OnComponentBeginOverlap`
  (params (OverlappedComponent :type "PrimitiveComponent Object Reference") (OtherActor :type "Actor Object Reference") (OtherComp :type "PrimitiveComponent Object Reference") (OtherBodyIndex :type Integer) (bFromSweep :type Boolean) (SweepResult :type "HitResult Structure (by ref)"))
  (bind _returnvalue_x (`KismetMathLibrary.BreakVector` (`SceneComponent.K2_GetComponentLocation` (`Actor.RootComponent` (`self.Second Hand`)))))
  (if (`self.FirstHandGrab`)
    (bind _asbp_motion_controller (cast `/Game/VirtualRealityBP/Blueprints/BP_MotionController` OtherActor))
    (if (!= (`/Game/VirtualRealityBP/Blueprints/BP_MotionController.MotionController` _asbp_motion_controller) (`self.First Hand`))
      (set `self.SecondHandGrab` true)
      (set `self.Second Hand` OtherActor)
      (`Timeline|Following Hand` :!via `PlayFromStart` :!label _label
        (:`Update`
          (if (`|EnumInequality` (`/Game/VirtualRealityBP/Blueprints/BP_MotionController.GripState` _asbp_motion_controller) "NewEnumerator0")
            (`SceneComponent.K2_SetWorldLocation` (`self.Slider_SM`) (`KismetMathLibrary.MakeVector` _returnvalue_x) false false)
            (else
              (goto _label :!via `Stop`))))
        (:`Finished`
          (`KismetSystemLibrary.MoveComponentTo` null (0.0 0.0 0.0) (struct) false false 0.1))))))

(event `/Game/Blueprints/Interfaces/BPI_GrabbableObj.Grab`
  (params (HandSocket :type Name) (AttachToMe :type "SceneComponent Object Reference"))
  ;[0 0 0] Grabbing
  (if (not (`self.FirstHandGrab`))
    (`/Game/Blueprints/GrabbableObjectSocket.Grab` (`self.GrabbableObjectSocket`) (`self.Firearm_SM`) self AttachToMe HandSocket)
    (`SceneComponent.K2_SetRelativeRotation` (`self.Firearm_SM`) (`self.OneHandRotation`) false false)
    (set `self.FirstHandGrab` true)
    (set `self.SecondHandGrab` false)
    (set `self.First Hand` AttachToMe)))

(event `/Game/VirtualRealityBP/Blueprints/PickupActorInterface.Drop`
  ;[0 0 0] Releasing
  (if (`self.FirstHandGrab`)
    (`/Game/Blueprints/GrabbableObjectSocket.Release` (`self.GrabbableObjectSocket`))
    (set `self.FirstHandGrab` false)
    (set `self.SecondHandGrab` false)))

(event `InputAction|PrimaryTriggerLeft`
  (params (Key :type "Key Structure"))
  ;[0 0 0] Player Input
  ;;[0.07819 0.07819 0.07819] Left Primary Trigger
  (:`Pressed`
    (if (`self.FirstHandGrab`)
      (switch `EControllerHand` (`self.dominantHand`)
        (:`Left`
          (set `self.isFiring` true)
          (switch `/Game/Blueprints/Enums/E_FireMode` (`self.currentFireMode`)
            (:`NewEnumerator0`
              (`self.Fire`))
            (:`NewEnumerator2`
              (`KismetSystemLibrary.K2_SetTimerDelegate` (delegate `Fire`) (`self.firerate`) (`self.isFiring`))))))))
  (:`Released`
    (set `self.isFiring` false)))

(event `InputAction|PrimaryTriggerRight`
  (params (Key :type "Key Structure"))
  ;[0 0 0] Player Input
  ;;[0.07819 0.07819 0.07819] Right Primary Trigger
  (:`Pressed`
    (if (`self.FirstHandGrab`)
      (switch `EControllerHand` (`self.dominantHand`)
        (:`Right`
          (set `self.isFiring` true)
          (switch `/Game/Blueprints/Enums/E_FireMode` (`self.currentFireMode`)
            (:`NewEnumerator0`
              (`self.Fire`))
            (:`NewEnumerator2`
              (`KismetSystemLibrary.K2_SetTimerDelegate` (delegate `Fire`) (`self.firerate`) (`self.isFiring`))))))))
  (:`Released`
    (set `self.isFiring` false)))

(event `InputAction|PrimaryButtonRight`
  (params (Key :type "Key Structure"))
  ;[0 0 0] Player Input
  ;;[0.07819 0.07819 0.07819] Right Primary Button
  (:`Pressed`
    (if (`self.FirstHandGrab`)
      (`self.Release Magazine`))))

(event `InputAction|SecondaryButtonRight`
  (params (Key :type "Key Structure"))
  ;[0 0 0] Player Input
  ;;[0.07819 0.07819 0.07819] Right Secondary Button
  (:`Pressed`
    (if (`self.FirstHandGrab`)
      (`self.Change Fire Mode`))))

(event `Fire`
  (bind _firearm_sm (`self.Firearm_SM`))
  (bind _returnvalue (`SceneComponent.K2_GetComponentLocation` _firearm_sm))
  ;[0 0 0] Firing
  (if (`self.canFire`)
    (if (`self.isLoaded`)
      (if (> (`self.currentAmmo`) 0)
        (if (< (`self.spentShells`) 1)
          (switch `/Game/Blueprints/Enums/E_LoadType` (`self.loadType`)
            (:`NewEnumerator0`
              _)
            (:`NewEnumerator1`
              (`/Engine/EditorBlueprintResources/StandardMacros.IncrementInt` (`self.spentShells`)
                (:`  `
                  _))))
          (`/Engine/EditorBlueprintResources/StandardMacros.DecrementInt` (`self.currentAmmo`)
            (:`  `
              (bind _outhit (`KismetSystemLibrary.LineTraceSingleForObjects` _returnvalue (+ _returnvalue (* (`KismetMathLibrary.GetForwardVector` (`SceneComponent.K2_GetComponentRotation` _firearm_sm)) 200)) (`|MakeArray` "ObjectTypeQuery7" "ObjectTypeQuery1" :!type "EObjectTypeQuery Enum")))
              (switch `ECollisionChannel` (`PrimitiveComponent.GetCollisionObjectType` (`.HitComponent` (`GameplayStatics.BreakHitResult` _outhit)))
                (:`ECC_WorldStatic`
                  (`KismetSystemLibrary.PrintString` "Gun hit Static Geo"))
                (:`ECC_GameTraceChannel1`
                  (`KismetSystemLibrary.PrintString` "Gun hit Enemy")
                  (message `/Game/Blueprints/Interfaces/BPI_TakeDamage.TakeDamage` (`.HitComponent` (`GameplayStatics.BreakHitResult` _outhit)) (`self.damageAmount`)))))))))))

(event `Change Fire Mode`
  ;[0 0 0] Changing Fire Mode
  (if (`self.canAutomatic`)
    (if (not (`self.isFiring`))
      (switch `/Game/Blueprints/Enums/E_FireMode` (`self.currentFireMode`)
        (:`NewEnumerator0`
          (set `self.currentFireMode` "NewEnumerator2"))
        (:`NewEnumerator2`
          (set `self.currentFireMode` "NewEnumerator0"))))))

(event `self.AmmoPortTrigger.OnComponentBeginOverlap`
  (params (OverlappedComponent :type "PrimitiveComponent Object Reference") (OtherActor :type "Actor Object Reference") (OtherComp :type "PrimitiveComponent Object Reference") (OtherBodyIndex :type Integer) (bFromSweep :type Boolean) (SweepResult :type "HitResult Structure (by ref)"))
  ;[0 0 0] Reloading
  (if (not (`self.isFiring`))
    (switch `/Game/Blueprints/Enums/E_LoadType` (`self.loadType`)
      (:`NewEnumerator0`
        ;;[0.07819 0.07819 0.07819] Magazine
        (bind _output_get (set `self.magazineObj` OtherActor))
        (bind _asbp_ammo_base (cast `/Game/Blueprints/Weapons/BP_AmmoBase` _output_get))
        (set `self.currentAmmo` (+ (`self.currentAmmo`) (`/Game/Blueprints/Weapons/BP_AmmoBase.currentAmmo` _asbp_ammo_base)))
        (`self.K2_AttachToComponent` _output_get null "None" "SnapToTarget" "SnapToTarget" "SnapToTarget" false)
        (set `self.isLoaded` true :!label _label_2))
      (:`NewEnumerator1`
        ;;[0.07819 0.07819 0.07819] Shells
        (if (< (`self.currentAmmo`) 6)
          (bind _result (`/Engine/EditorBlueprintResources/StandardMacros.IncrementInt` (`self.currentAmmo`))
            (:`  `
              (`self.K2_DestroyActor` OtherActor)
              (if (> _result 0)
                (goto _label_2)))))))))

(event `Release Magazine`
  (bind _magazineobj (`self.magazineObj`))
  ;[0 0 0] Ammo Ejection
  (if (not (`self.isFiring`))
    (switch `/Game/Blueprints/Enums/E_LoadType` (`self.loadType`)
      (:`NewEnumerator0`
        ;;[0.07819 0.07819 0.07819] Magazine
        (set `self.currentAmmo` 0)
        (`self.K2_DetachFromActor` _magazineobj "KeepWorld" "KeepWorld" "KeepWorld")
        (bind _asbp_ammo_base (cast `/Game/Blueprints/Weapons/BP_AmmoBase` _magazineobj))
        (`PrimitiveComponent.SetSimulatePhysics` (`/Game/Blueprints/Weapons/BP_AmmoBase.Ammo_SM` _asbp_ammo_base) true)
        (set `self.isLoaded` false :!label _label_3))
      (:`NewEnumerator1`
        ;;[0.07819 0.07819 0.07819] Shells
        (if (> (`self.spentShells`) 0)
          (bind _result (`/Engine/EditorBlueprintResources/StandardMacros.DecrementInt` (`self.spentShells`))
            (:`  `
              (if (< _result 1)
                (if (< (`self.currentAmmo`) 1)
                  (goto _label_3))))))))))

(fn `UserConstructionScript`)