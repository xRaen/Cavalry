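; VR-style grabbable firearm Blueprint with single and optional automatic fire, supporting magazine or shell loading.
; The dominant hand's trigger runs Fire, which spends ammo and line-traces a short distance forward, sending damage to enemy hits.
; Overlapping the ammo port attaches a magazine or consumes a shell.
; Right-hand buttons toggle fire mode and release the magazine or clear the spent shell that blocks the next shot.
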(event `InputAction|PrimaryTriggerLeft`
  (params (Key :type "Key Structure"))
  ;[0 0 0] Player Input
  ;;[0.07819 0.07819 0.07819] Left Primary Trigger
  (:`Pressed`
    (if (`self.isGrabbed`)
      (switch `/Game/Blueprints/Enums/E_Hands` (`self.dominantHand`)
        (:`NewEnumerator1`
          (set `self.isFiring` true)
          (switch `/Game/Blueprints/Enums/E_FireMode` (`self.currentFireMode`)
            (:`NewEnumerator0`
              (`self.Fire`))
            (:`NewEnumerator2`
              (`KismetSystemLibrary.K2_SetTimerDelegate` (delegate `Fire`) (`self.firerate`) (`self.isFiring`))))))))
  (:`Released`
    (set `self.isFiring` false)))

(event `InputAction|PrimaryTriggerRight`
  (params (Key :type "Key Structure"))
  ;[0 0 0] Player Input
  ;;[0.07819 0.07819 0.07819] Right Primary Trigger
  (:`Pressed`
    (if (`self.isGrabbed`)
      (switch `/Game/Blueprints/Enums/E_Hands` (`self.dominantHand`)
        (:`NewEnumerator0`
          (set `self.isFiring` true)
          (switch `/Game/Blueprints/Enums/E_FireMode` (`self.currentFireMode`)
            (:`NewEnumerator0`
              (`self.Fire`))
            (:`NewEnumerator2`
              (`KismetSystemLibrary.K2_SetTimerDelegate` (delegate `Fire`) (`self.firerate`) (`self.isFiring`))))))))
  (:`Released`
    (set `self.isFiring` false)))

(event `InputAction|PrimaryButtonRight`
  (params (Key :type "Key Structure"))
  ;[0 0 0] Player Input
  ;;[0.07819 0.07819 0.07819] Right Primary Button
  (:`Pressed`
    (if (`self.isGrabbed`)
      (`self.Release Magazine`))))

(event `InputAction|SecondaryButtonRight`
  (params (Key :type "Key Structure"))
  ;[0 0 0] Player Input
  ;;[0.07819 0.07819 0.07819] Right Secondary Button
  (:`Pressed`
    (if (`self.isGrabbed`)
      (`self.Change Fire Mode`))))

(event `Fire`
  (bind _skm_firearm (`self.SkM_Firearm`))
  (bind _returnvalue (`SceneComponent.K2_GetComponentLocation` _skm_firearm))
  ;[0 0 0] Firing
  (if (`self.canFire`)
    (if (`self.isLoaded`)
      (if (> (`self.currentAmmo`) 0)
        (if (< (`self.spentShells`) 1)
          (switch `/Game/Blueprints/Enums/E_LoadType` (`self.loadType`)
            (:`NewEnumerator0`
              _)
            (:`NewEnumerator1`
              (`/Engine/EditorBlueprintResources/StandardMacros.IncrementInt` (`self.spentShells`)
                (:`  `
                  _))))
          (`/Engine/EditorBlueprintResources/StandardMacros.DecrementInt` (`self.currentAmmo`)
            (:`  `
              (bind _outhit (`KismetSystemLibrary.LineTraceSingleForObjects` _returnvalue (+ _returnvalue (* (`KismetMathLibrary.GetForwardVector` (`SceneComponent.K2_GetComponentRotation` _skm_firearm)) 200)) (`|MakeArray` "ObjectTypeQuery7" "ObjectTypeQuery1" :!type "EObjectTypeQuery Enum")))
              (switch `ECollisionChannel` (`PrimitiveComponent.GetCollisionObjectType` (`.HitComponent` (`GameplayStatics.BreakHitResult` _outhit)))
                (:`ECC_WorldStatic`
                  (`KismetSystemLibrary.PrintString` "Gun hit Static Geo"))
                (:`ECC_GameTraceChannel1`
                  (`KismetSystemLibrary.PrintString` "Gun hit Enemy")
                  (message `/Game/Blueprints/Interfaces/BPI_TakeDamage.TakeDamage` (`.HitComponent` (`GameplayStatics.BreakHitResult` _outhit)) (`self.damageAmount`)))))))))))

(event `Change Fire Mode`
  ;[0 0 0] Changing Fire Mode
  (if (`self.canAutomatic`)
    (if (not (`self.isFiring`))
      (switch `/Game/Blueprints/Enums/E_FireMode` (`self.currentFireMode`)
        (:`NewEnumerator0`
          (set `self.currentFireMode` "NewEnumerator2"))
        (:`NewEnumerator2`
          (set `self.currentFireMode` "NewEnumerator0"))))))

(event `self.AmmoPortTrigger.OnComponentBeginOverlap`
  (params (OverlappedComponent :type "PrimitiveComponent Object Reference") (OtherActor :type "Actor Object Reference") (OtherComp :type "PrimitiveComponent Object Reference") (OtherBodyIndex :type Integer) (bFromSweep :type Boolean) (SweepResult :type "HitResult Structure (by ref)"))
  ;[0 0 0] Reloading
  (if (not (`self.isFiring`))
    (switch `/Game/Blueprints/Enums/E_LoadType` (`self.loadType`)
      (:`NewEnumerator0`
        ;;[0.07819 0.07819 0.07819] Magazine
        (bind _output_get (set `self.magazineObj` OtherActor))
        (bind _asbp_ammo_base (cast `/Game/Blueprints/Weapons/BP_AmmoBase` _output_get))
        (set `self.currentAmmo` (+ (`self.currentAmmo`) (`/Game/Blueprints/Weapons/BP_AmmoBase.currentAmmo` _asbp_ammo_base)))
        (`self.K2_AttachToComponent` _output_get null "None" "SnapToTarget" "SnapToTarget" "SnapToTarget" false)
        (set `self.isLoaded` true :!label _label))
      (:`NewEnumerator1`
        ;;[0.07819 0.07819 0.07819] Shells
        (if (< (`self.currentAmmo`) 6)
          (bind _result (`/Engine/EditorBlueprintResources/StandardMacros.IncrementInt` (`self.currentAmmo`))
            (:`  `
              (`self.K2_DestroyActor` OtherActor)
              (if (> _result 0)
                (goto _label)))))))))

(event `Release Magazine`
  (bind _magazineobj (`self.magazineObj`))
  ;[0 0 0] Ammo Ejection
  (if (not (`self.isFiring`))
    (switch `/Game/Blueprints/Enums/E_LoadType` (`self.loadType`)
      (:`NewEnumerator0`
        ;;[0.07819 0.07819 0.07819] Magazine
        (set `self.currentAmmo` 0)
        (`self.K2_DetachFromActor` _magazineobj "KeepWorld" "KeepWorld" "KeepWorld")
        (bind _asbp_ammo_base (cast `/Game/Blueprints/Weapons/BP_AmmoBase` _magazineobj))
        (`PrimitiveComponent.SetSimulatePhysics` (`/Game/Blueprints/Weapons/BP_AmmoBase.Ammo_SM` _asbp_ammo_base) true)
        (set `self.isLoaded` false :!label _label_2))
      (:`NewEnumerator1`
        ;;[0.07819 0.07819 0.07819] Shells
        (if (> (`self.spentShells`) 0)
          (bind _result (`/Engine/EditorBlueprintResources/StandardMacros.DecrementInt` (`self.spentShells`))
            (:`  `
              (if (< _result 1)
                (if (< (`self.currentAmmo`) 1)
                  (goto _label_2))))))))))

(event `SlideRelease`
  ;[0 0 0] Slider Release & Snap
  (`KismetSystemLibrary.MoveComponentTo` (`self.SkM_Slider`) (0.0 0.0 0.0) (struct) false false 0.1))

(fn `UserConstructionScript`)