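; VR shotgun Blueprint that handles two-handed gripping and a sliding pump driven by motion controllers.
; The first grab attaches the firearm via its grabbable socket; a second grab snaps that hand's mesh to the second-hand socket.
; A timeline then aims the gun at the second controller and moves the slider by its local X motion within limits.
; Changing grip state or clearing the second-hand flag releases that hand and stops the timeline.
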(event `self.SliderRevertPosition`
  ;[1 1 1] Slider Reset
  (set `self.SecondHandGrabbed` false))

(event `/Game/Blueprints/Interfaces/BPI_GrabbableObj.Grab`
  (params (HandSocket :type Name) (AttachToMe :type "SceneComponent Object Reference") (Actor :type "Actor Object Reference"))
  (bind _x_last_position_x (`KismetMathLibrary.BreakVector` (`self.X_Last_Position`)))
  (bind _slider_sm (`self.Slider_SM`))
  (bind _x_last_position_x_2 (`KismetMathLibrary.BreakVector` (`self.X_Last_Position`)))
  (bind _returnvalue_location (`KismetMathLibrary.BreakTransform` (`SceneComponent.K2_GetComponentToWorld` (`self.Firearm_SM`))))
  (bind _relativelocation_x (`KismetMathLibrary.BreakVector` (`SceneComponent.RelativeLocation` _slider_sm)))
  (bind _relativelocation_x_2 (`KismetMathLibrary.BreakVector` (`SceneComponent.RelativeLocation` _slider_sm)))
  (bind _returnvalue_x (`KismetMathLibrary.BreakVector` (`KismetMathLibrary.InverseTransformLocation` (`SceneComponent.K2_GetComponentToWorld` (`self.Firearm_SM`)) (`SceneComponent.K2_GetComponentLocation` (`/Game/VirtualRealityBP/Blueprints/BP_MotionController.MotionController` (`self.Second Hand Motion Controller`))))))
  (bind _returnvalue_x_2 (`KismetMathLibrary.BreakVector` (`KismetMathLibrary.InverseTransformLocation` (`SceneComponent.K2_GetComponentToWorld` (`self.Firearm_SM`)) (`SceneComponent.K2_GetComponentLocation` (`/Game/VirtualRealityBP/Blueprints/BP_MotionController.MotionController` (`self.Second Hand Motion Controller`))))))
  ;[1 1 1] Comment
  (if (`self.FirstHandGrabbed`)
    ;;[0.1333 0.1333 0.1333] Slider Grab
    (set `self.SecondHandGrabbed` true)
    (`SceneComponent.K2_AttachToComponent` AttachToMe (`self.Firearm_SM`) "Second_Hand_Socket" "SnapToTarget" "SnapToTarget" "KeepWorld" true)
    (bind _asbp_motion_controller (cast `/Game/VirtualRealityBP/Blueprints/BP_MotionController` Actor))
    (bind _output_get (set `self.Second Hand Motion Controller` _asbp_motion_controller))
    (set `self.Second Hand Mesh` AttachToMe)
    (set `self.X_Last_Position` (`KismetMathLibrary.MakeVector` _returnvalue_x_2))
    (set `/Game/VirtualRealityBP/Blueprints/BP_MotionController.GripState` "NewEnumerator3" _output_get)
    (`Timeline|Timeline_1` :!via `PlayFromStart` :!label _label
      (:`Update`
        (if (`|EnumInequality` (`/Game/VirtualRealityBP/Blueprints/BP_MotionController.GripState` (`self.Second Hand Motion Controller`)) "NewEnumerator0")
          (if (`self.SecondHandGrabbed`)
            (bind _output_get_2 (set `self.X_Delta` (- _returnvalue_x _x_last_position_x)))
            (set `self.X_Last_Position` (`KismetMathLibrary.MakeVector` (+ _output_get_2 _x_last_position_x_2)))
            (`SceneComponent.K2_AddRelativeLocation` _slider_sm (`KismetMathLibrary.MakeVector` _output_get_2) true true)
            (`SceneComponent.K2_SetWorldRotation` (`self.Firearm_SM`) (`KismetMathLibrary.FindLookAtRotation` _returnvalue_location (`SceneComponent.K2_GetComponentLocation` (`/Game/VirtualRealityBP/Blueprints/BP_MotionController.MotionController` (`self.Second Hand Motion Controller`)))) false false)
            (if (> _relativelocation_x_2 (`self.SliderXMax`))
              (`SceneComponent.K2_SetRelativeLocation` _slider_sm (0.0 0.0 0.0) false false)
              (elif (< _relativelocation_x (`self.SliderXMin`))
                (`SceneComponent.K2_SetRelativeLocation` _slider_sm (-10.0 0.0 0.0) false false)))
            (else
              (`self.SliderRevertPosition` :!label _label_2)
              (`self.SecondHandRelease`)
              (goto _label :!via `Stop`)))
          (else
            (goto _label_2)))))
    (else
      ;;[0.1771 0.1771 0.1771] First Hand Grabbed
      (`/Game/Blueprints/GrabbableObjectSocket.Grab` (`self.GrabbableObjectSocket`) (`self.Firearm_SM`) self HandSocket AttachToMe)
      (set `self.FirstHandGrabbed` true)
      (set `self.SecondHandGrabbed` false)
      (set `self.First Hand` AttachToMe)
      (bind _asbp_motion_controller_2 (cast `/Game/VirtualRealityBP/Blueprints/BP_MotionController` Actor))
      (set `self.dominantHand` (`/Game/VirtualRealityBP/Blueprints/BP_MotionController.Hand` _asbp_motion_controller_2))
      (set `/Game/VirtualRealityBP/Blueprints/BP_MotionController.GripState` "NewEnumerator2" _asbp_motion_controller_2))))

(fn `UserConstructionScript`
  (`parent.UserConstructionScript`))