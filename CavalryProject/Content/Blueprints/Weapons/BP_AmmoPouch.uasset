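; BP_AmmoPouch is a grabbable VR ammo pouch that snaps to magnetic mounts and dispenses magazines.
; Grabbing it while mounted spawns a magazine into the motion controller's hand and decrements the count; otherwise the pouch itself is picked up through GrabbableObjectSocket.
; On release, it attaches to the closest unoccupied, type-compatible BP_MagneticPlacement among those tracked by its collision overlaps, disabling physics and marking that mount occupied.
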(event `/Game/Blueprints/Interfaces/BPI_GrabbableObj.Grab`
  (params (HandSocket :type Name) (AttachToMe :type "SceneComponent Object Reference") (Actor :type "Actor Object Reference"))
  ;[0 0 0] Grabbing
  (if (`self.OnMagnetMount`)
    (if (> (`self.MagCount`) 0)
      (bind _returnvalue (`|SpawnActorFromClass` (`self.MagType`) (`KismetMathLibrary.MakeTransform` (0.0 0.0 0.0)) "Undefined" "OverrideRootScale" null 1 null))
      (message `/Game/Blueprints/Interfaces/BPI_GrabbableObj.Grab` _returnvalue HandSocket AttachToMe Actor)
      (`/Engine/EditorBlueprintResources/StandardMacros.DecrementInt` (`self.MagCount`)
        (:`  `
          (bind _asbp_motion_controller (cast `/Game/VirtualRealityBP/Blueprints/BP_MotionController` Actor))
          (set `/Game/VirtualRealityBP/Blueprints/BP_MotionController.AttachedActor` _returnvalue _asbp_motion_controller))))
    (else
      (`/Game/Blueprints/GrabbableObjectSocket.Grab` (`self.GrabbableObjectSocket`) (`self.Ammo_SM`) self HandSocket AttachToMe)
      (set `self.IsGrabbed` true)
      (if (`self.OnMagnetMount`)
        (set `/Game/Blueprints/Tools/BP_MagneticPlacement.Occupied` false (`self.MagnetMount`))
        (set `self.OnMagnetMount` false)))))

(event `/Game/Blueprints/Interfaces/BPI_GrabbableObj.Release`
  (params (NewParam :type "EControllerHand Enum" :default "Left"))
  ;[0 0 0] Releasing
  (`/Game/Blueprints/GrabbableObjectSocket.Release` (`self.GrabbableObjectSocket`))
  (set `self.IsGrabbed` false)
  (if (not (== (`KismetArrayLibrary.Array_Length` (`self.OverlappingMagnets`)) 0))
    (`self.Magnetize` (`|GetArrayItem` (`self.OverlappingMagnets`)))))

(event `self.Magnetize`
  (params (Magnet :type "Actor Object Reference"))
  (bind _ammo_sm (`self.Ammo_SM`))
  (bind _closestmount (`self.ClosestMount`))
  (bind _returnvalue (`SceneComponent.K2_GetComponentLocation` (`self.MagnetCollision`)))
  ;[0 0 0] Magnetic
  (if (`self.InGun`)
    _
    (elif (not (`self.IsGrabbed`))
      (set `self.ClosestMount` null)
      (for _array_element (`self.OverlappingMagnets`)
        (if (`/Game/Blueprints/Tools/BP_MagneticPlacement.Occupied` _array_element)
          _
          (elif (or (`|EnumEquality` (`self.Ammo Object Type`) (`/Game/Blueprints/Tools/BP_MagneticPlacement.Object Type` _array_element)) (`|EnumEquality` (`/Game/Blueprints/Tools/BP_MagneticPlacement.Object Type` _array_element) "NewEnumerator0"))
            (if (`KismetSystemLibrary.IsValid` (`self.ClosestMount`))
              (if (< (`KismetMathLibrary.VSize` (- _returnvalue (`SceneComponent.K2_GetComponentLocation` (`Actor.RootComponent` _array_element)))) (`KismetMathLibrary.VSize` (- _returnvalue (`SceneComponent.K2_GetComponentLocation` (`Actor.RootComponent` (`self.ClosestMount`))))))
                (set `self.ClosestMount` _array_element))
              (else
                (set `self.ClosestMount` _array_element))))))
      (if (`KismetSystemLibrary.IsValid` (`self.ClosestMount`))
        (`PrimitiveComponent.SetSimulatePhysics` _ammo_sm false)
        (`SceneComponent.K2_AttachToComponent` _ammo_sm (`Actor.RootComponent` _closestmount) "None" "SnapToTarget" "SnapToTarget" "KeepWorld" false)
        (set `self.OnMagnetMount` true)
        (bind _output_get (set `self.MagnetMount` _closestmount))
        (set `/Game/Blueprints/Tools/BP_MagneticPlacement.Occupied` true _output_get)))))

(event `self.MagnetCollision.OnComponentBeginOverlap`
  (params (OverlappedComponent :type "PrimitiveComponent Object Reference") (OtherActor :type "Actor Object Reference") (OtherComp :type "PrimitiveComponent Object Reference") (OtherBodyIndex :type Integer) (bFromSweep :type Boolean) (SweepResult :type "HitResult Structure (by ref)"))
  ;[0 0 0] Magnetic
  (bind _asbp_magnetic_placement (cast `/Game/Blueprints/Tools/BP_MagneticPlacement` OtherActor))
  (`KismetArrayLibrary.Array_Add` (`self.OverlappingMagnets`) _asbp_magnetic_placement))

(event `self.MagnetCollision.OnComponentEndOverlap`
  (params (OverlappedComponent :type "PrimitiveComponent Object Reference") (OtherActor :type "Actor Object Reference") (OtherComp :type "PrimitiveComponent Object Reference") (OtherBodyIndex :type Integer))
  ;[0 0 0] Magnetic
  (bind _asbp_magnetic_placement (cast `/Game/Blueprints/Tools/BP_MagneticPlacement` OtherActor))
  (`KismetArrayLibrary.Array_RemoveItem` (`self.OverlappingMagnets`) _asbp_magnetic_placement))

(fn `UserConstructionScript`)