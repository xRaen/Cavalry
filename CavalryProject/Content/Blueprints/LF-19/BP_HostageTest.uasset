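; BP_HostageTest is a test hostage actor that a player rescues by touching it.
; An overlap or hit on its static mesh by an actor tagged "Player" triggers the rescue.
; Both contact events share one path that hides the mesh, disables its collision and calls HostageRescuedMessage on the game state.
; The actor is disabled in place rather than destroyed.
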(event `self.Hostage_SM.OnComponentBeginOverlap`
  (params (OverlappedComponent :type "PrimitiveComponent Object Reference") (OtherActor :type "Actor Object Reference") (OtherComp :type "PrimitiveComponent Object Reference") (OtherBodyIndex :type Integer) (bFromSweep :type Boolean) (SweepResult :type "HitResult Structure (by ref)"))
  ;[0 0 0] Did a player touch the hostage
  (if (`self.ActorHasTag` OtherActor "Player")
    (`self.DisableHostage` :!label _label)
    (message `/Game/Blueprints/Interfaces/BPI_GameStateCommunication.HostageRescued` (`GameplayStatics.GetGameState`))))

(event `self.Hostage_SM.OnComponentHit`
  (params (HitComponent :type "PrimitiveComponent Object Reference") (OtherActor :type "Actor Object Reference") (OtherComp :type "PrimitiveComponent Object Reference") (NormalImpulse :type "Vector Structure") (Hit :type "HitResult Structure (by ref)"))
  ;[0 0 0] Did a player touch the hostage
  (if (`self.ActorHasTag` OtherActor "Player")
    (goto _label)))

(event `DisableHostage`
  (bind _hostage_sm (`self.Hostage_SM`))
  ;[0 0 0] Disable the hostage
  (`SceneComponent.SetVisibility` _hostage_sm false false)
  (`PrimitiveComponent.SetCollisionEnabled` _hostage_sm "NoCollision"))

(fn `UserConstructionScript`)