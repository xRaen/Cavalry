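; Powered sliding door that toggles open and closed when something overlaps its access pad while it is unlocked.
; A timeline slides the mesh along Y, with a DoOnce and delay limiting retriggers, while two placeholder texts flash red or green for lock state.
; Events set lock and power, the latter gated by CanBePoweredOff.
; Grab is empty; motion-controller hand-sliding logic for an unpowered door is disconnected.
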(event `/Game/Blueprints/Interfaces/BPI_GrabbableObj.Grab`
  (params (HandSocket :type Name) (AttachToMe :type "SceneComponent Object Reference") (Actor :type "Actor Object Reference")))

(event `self.AccessPad_SM.OnComponentBeginOverlap`
  (params (OverlappedComponent :type "PrimitiveComponent Object Reference") (OtherActor :type "Actor Object Reference") (OtherComp :type "PrimitiveComponent Object Reference") (OtherBodyIndex :type Integer) (bFromSweep :type Boolean) (SweepResult :type "HitResult Structure (by ref)"))
  (if (`self.IsPowered`)
    (if (`self.IsLocked`)
      (`self.PlaceholderTextChange`)
      (`self.Placeholdertextchange2`)
      (else
        (`self.PlaceholderTextChange`)
        (`self.Placeholdertextchange2`)
        (`KismetSystemLibrary.PrintString` "Door ACTIVATED")
        (`/Engine/EditorBlueprintResources/StandardMacros.DoOnce` false :!label _label
          (:`Completed`
            (if (`self.IsClosed`)
              (`self.DoorOpen`)
              (set `self.IsClosed` false)
              (else
                (`self.DoorClose`)
                (set `self.IsClosed` true)))
            (`KismetSystemLibrary.Delay` 1.0)
            (goto _label :!via `Reset`)))))))

(event `DoorOpen`
  (bind (_direction _y_lerp) (`Timeline|DoorOpenTimeline` :!label _label_2)
    (:`Update`
      (`SceneComponent.K2_SetRelativeLocation` (`self.Door_SM`) (`KismetMathLibrary.MakeVector` 0.0 (`KismetMathLibrary.Lerp` 0.0 -210.0 _y_lerp)) false false))))

(event `DoorClose`
  (goto _label_2 :!via `Reverse`))

(event `PowerOn`
  ;[0 0 0] Used by the Level Blueprint
  (if (`self.CanBePoweredOff`)
    (set `self.IsPowered` true)))

(event `PowerOff`
  ;[0 0 0] Used by the Level Blueprint
  (if (`self.CanBePoweredOff`)
    (set `self.IsPowered` false)))

(event `LockDoor`
  (set `self.IsLocked` true))

(event `UnlockDoor`
  (set `self.IsLocked` false))

(event `PlaceholderTextChange`
  ;[0 0 0] PLACEHOLDER AND WILL BE DELETED WHEN WE DO ART PASS
  (`/Engine/EditorBlueprintResources/StandardMacros.DoOnce` false :!label _label_3
    (:`Completed`
      (if (`self.IsLocked`)
        ;;[0.07292 0.07292 0.07292] This section should replaced with a material
        (`TextRenderComponent.SetTextRenderColor` (`self.PLACEHOLDERTEXT`) (make `Color` 0 0 255 255))
        (`KismetSystemLibrary.Delay` 0.3)
        (`TextRenderComponent.SetTextRenderColor` (`self.PLACEHOLDERTEXT`) (make `Color` 255 255 255 255))
        (`TextRenderComponent.SetTextRenderColor` (`self.PLACEHOLDERTEXT`) (make `Color` 0 0 255 255))
        (`KismetSystemLibrary.Delay` 0.3)
        (`TextRenderComponent.SetTextRenderColor` (`self.PLACEHOLDERTEXT`) (make `Color` 255 255 255 255))
        (`TextRenderComponent.SetTextRenderColor` (`self.PLACEHOLDERTEXT`) (make `Color` 0 0 255 255))
        (`KismetSystemLibrary.Delay` 0.3)
        (`TextRenderComponent.SetTextRenderColor` (`self.PLACEHOLDERTEXT`) (make `Color` 255 255 255 255))
        (goto _label_3 :!via `Reset`)
        (else
          (`TextRenderComponent.SetTextRenderColor` (`self.PLACEHOLDERTEXT`) (make `Color` 0 255 0 255))
          (`KismetSystemLibrary.Delay` 1.0)
          (`TextRenderComponent.SetTextRenderColor` (`self.PLACEHOLDERTEXT`) (make `Color` 255 255 255 255))
          (goto _label_3 :!via `Reset`))))))

(event `Placeholdertextchange2`
  ;[0 0 0] PLACEHOLDER AND WILL BE DELETED WHEN WE DO ART PASS
  (`/Engine/EditorBlueprintResources/StandardMacros.DoOnce` false :!label _label_4
    (:`Completed`
      (if (`self.IsLocked`)
        ;;[0.07292 0.07292 0.07292] This section should replaced with a material
        (`TextRenderComponent.SetTextRenderColor` (`self.PLACEHOLDERTEXT1`) (make `Color` 0 0 255 255))
        (`KismetSystemLibrary.Delay` 0.3)
        (`TextRenderComponent.SetTextRenderColor` (`self.PLACEHOLDERTEXT1`) (make `Color` 255 255 255 255))
        (`TextRenderComponent.SetTextRenderColor` (`self.PLACEHOLDERTEXT1`) (make `Color` 0 0 255 255))
        (`KismetSystemLibrary.Delay` 0.3)
        (`TextRenderComponent.SetTextRenderColor` (`self.PLACEHOLDERTEXT1`) (make `Color` 255 255 255 255))
        (`TextRenderComponent.SetTextRenderColor` (`self.PLACEHOLDERTEXT1`) (make `Color` 0 0 255 255))
        (`KismetSystemLibrary.Delay` 0.3)
        (`TextRenderComponent.SetTextRenderColor` (`self.PLACEHOLDERTEXT1`) (make `Color` 255 255 255 255))
        (goto _label_4 :!via `Reset`)
        (else
          (`TextRenderComponent.SetTextRenderColor` (`self.PLACEHOLDERTEXT1`) (make `Color` 0 255 0 255))
          (`KismetSystemLibrary.Delay` 1.0)
          (`TextRenderComponent.SetTextRenderColor` (`self.PLACEHOLDERTEXT1`) (make `Color` 255 255 255 255))
          (goto _label_4 :!via `Reset`))))))

(fn `UserConstructionScript`)