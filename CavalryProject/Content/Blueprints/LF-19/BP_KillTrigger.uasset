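; BP_KillTrigger is a kill volume that kills the player character and moves it to the nearest BP_DeathPoint.
; It caches all death points on BeginPlay.
; An overlap on its collision component calls Death on the player, scans the cached points by distance, printing each new closest, then moves the player to the winner.
; The closest-distance variable carries over between overlaps, as the graph never resets it.
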(event `self.ReceiveBeginPlay`
  (bind _outactors (`GameplayStatics.GetAllActorsOfClass` "/Game/Blueprints/LF-19/BP_DeathPoint.BP_DeathPoint_C"))
  (set `self.DeathPoints` _outactors))

(event `self.CollisionComponent.OnComponentBeginOverlap`
  (params (OverlappedComponent :type "PrimitiveComponent Object Reference") (OtherActor :type "Actor Object Reference") (OtherComp :type "PrimitiveComponent Object Reference") (OtherBodyIndex :type Integer) (bFromSweep :type Boolean) (SweepResult :type "HitResult Structure (by ref)"))
  ;[0 0 0] Kill the player and teleport it to the nearest death point actor
  (bind _asbp_player_character_base (cast `/Game/Blueprints/Characters/BP_PlayerCharacter_Base` OtherActor))
  (`/Game/Blueprints/Characters/BP_PlayerCharacter_Base.Death` _asbp_player_character_base)
  (for _array_element (`self.DeathPoints`)
    (bind _returnvalue (`self.GetDistanceTo` _array_element OtherActor))
    (if (<= _returnvalue (`self.ClosestDistance`))
      (`KismetSystemLibrary.PrintString` (`KismetStringLibrary.Conv_DoubleToString` _returnvalue))
      (set `self.ClosestDistance` _returnvalue)
      (set `self.ClosestDeathPoint` _array_element)))
  (`self.K2_SetActorLocation` OtherActor (`self.K2_GetActorLocation` (`self.ClosestDeathPoint`)) false false))

(fn `UserConstructionScript`)