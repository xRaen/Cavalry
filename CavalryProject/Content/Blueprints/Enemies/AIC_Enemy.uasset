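; Enemy AI controller that runs BT_Enemy on possession, seeding its blackboard with reserved-cover and alive state.
; PawnSensing sight of players or heard noise sets TargetActor, enters combat and notifies the pawn.
; It alerts previously seen enemies not yet fighting, though the hearing path passes no target.
; Darkness events toggle sight radius, and RemoveAsTarget bindings on the four horseman player characters clear them as target.
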(event `self.ReceivePossess`
  (params (PossessedPawn :type "Pawn Object Reference"))
  ;[0 0 0] Behavior Tree Selection
  (`self.RunBehaviorTree` "/Game/Blueprints/Enemies/BT_Enemy.BT_Enemy")
  (bind _returnvalue (`GameplayStatics.GetActorOfClass` "/Game/Blueprints/Enemies/BP_ReservedCover.BP_ReservedCover_C"))
  (`BlackboardComponent.SetValueAsObject` (`self.Blackboard`) "ReservedCoverArray" _returnvalue)
  (`BlackboardComponent.SetValueAsBool` (`self.Blackboard`) "IsAlive" true)
  (set `self.Possessed Pawn` PossessedPawn)
  (bind _returnvalue_2 (`GameplayStatics.GetActorOfClass` "/Game/Blueprints/Characters/BPC_Conquest.BPC_Conquest_C"))
  ;[0 0 0] These 4 casts are for confirmation that a player with that character is in the level, don't worry about unreal saying we don't need it
  (bind _asbpc_conquest (cast `/Game/Blueprints/Characters/BPC_Conquest` _returnvalue_2)
    (:`then`
      (bind _output_get (set `self.PlayerConquest` _asbpc_conquest))
      (add `/Game/Blueprints/Characters/BP_PlayerCharacter_Base.RemoveAsTarget` _output_get (delegate `RemoveAsTarget_Conquest`)))
    (:`CastFailed`
      _))
  (bind _returnvalue_3 (`GameplayStatics.GetActorOfClass` "/Game/Blueprints/Characters/BPC_War.BPC_War_C"))
  (bind _asbpc_war (cast `/Game/Blueprints/Characters/BPC_War` _returnvalue_3)
    (:`then`
      (bind _output_get_2 (set `self.PlayerWar` _asbpc_war))
      (add `/Game/Blueprints/Characters/BP_PlayerCharacter_Base.RemoveAsTarget` _output_get_2 (delegate `RemoveAsTarget_War`)))
    (:`CastFailed`
      _))
  (bind _returnvalue_4 (`GameplayStatics.GetActorOfClass` "/Game/Blueprints/Characters/BPC_Famine.BPC_Famine_C"))
  (bind _asbpc_famine (cast `/Game/Blueprints/Characters/BPC_Famine` _returnvalue_4)
    (:`then`
      (bind _output_get_3 (set `self.PlayerFamine` _asbpc_famine))
      (add `/Game/Blueprints/Characters/BP_PlayerCharacter_Base.RemoveAsTarget` _output_get_3 (delegate `RemoveAsTarget_Famine`)))
    (:`CastFailed`
      _))
  (bind _returnvalue_5 (`GameplayStatics.GetActorOfClass` "/Game/Blueprints/Characters/BPC_Death.BPC_Death_C"))
  (bind _asbpc_death (cast `/Game/Blueprints/Characters/BPC_Death` _returnvalue_5))
  (bind _output_get_4 (set `self.PlayerDeath` _asbpc_death))
  (add `/Game/Blueprints/Characters/BP_PlayerCharacter_Base.RemoveAsTarget` _output_get_4 (delegate `RemoveAsTarget_Death`)))

(event `self.PawnSensing.OnSeePawn`
  (params (Pawn :type "Pawn Object Reference"))
  (bind _perceivedactor (`self.PerceivedActor`))
  ;[0 0 0] Player Targeting
  ;;[0.08235 0.08235 0.08235] Do we see an Actor with the Tag of Player?
  (set `self.PerceivedActor` Pawn)
  (if (`self.ActorHasTag` Pawn "Player")
    (`self.UpdateTargetKey` _perceivedactor)
    (set `self.InCombat` true)
    (`self.AlertNearby` _perceivedactor)
    (bind _asbp_enemy_base (cast `/Game/Blueprints/Enemies/BP_EnemyBase` (`self.Possessed Pawn`)))
    (`/Game/Blueprints/Enemies/BP_EnemyBase.PlayerSpotted` _asbp_enemy_base)
    (elif (`self.ActorHasTag` Pawn "Enemy")
      (`KismetArrayLibrary.Array_AddUnique` (`self.NearbyAIArray`) (`self.PerceivedActor`)))))

(event `AlertNearby`
  (params (Actor :type "Actor Object Reference"))
  ;[0 0 0] Alert other AI nearby to the presence of a target
  (for _array_element (`self.NearbyAIArray`)
    (bind _asbp_enemy_base (cast `/Game/Blueprints/Enemies/BP_EnemyBase` _array_element))
    (bind _asaic_enemy (cast `/Game/Blueprints/Enemies/AIC_Enemy` (`AIBlueprintHelperLibrary.GetAIController` _asbp_enemy_base)))
    (if (not (`/Game/Blueprints/Enemies/AIC_Enemy.InCombat` _asaic_enemy))
      (`self.Alert` _asaic_enemy Actor)
      (set `/Game/Blueprints/Enemies/AIC_Enemy.InCombat` true _asaic_enemy))))

(event `LowerSightRadius`
  ;[0 0 0] Lower sight when told its in darkness or smoke
  (set `PawnSensingComponent.SightRadius` 500.0 (`self.PawnSensing`))
  (bind _asbp_enemy_base (cast `/Game/Blueprints/Enemies/BP_EnemyBase` (`self.Possessed Pawn`)))
  (set `/Game/Blueprints/Enemies/BP_EnemyBase.InDarkness` true _asbp_enemy_base))

(event `ResetSightRadius`
  ;[0 0 0] Reset the sight radius
  (set `PawnSensingComponent.SightRadius` 2500.0 (`self.PawnSensing`))
  (bind _asbp_enemy_base (cast `/Game/Blueprints/Enemies/BP_EnemyBase` (`self.Possessed Pawn`)))
  (set `/Game/Blueprints/Enemies/BP_EnemyBase.InDarkness` false _asbp_enemy_base))

(event `self.PawnSensing.OnHearNoise`
  (params (Instigator :type "Pawn Object Reference") (Location :type "Vector Structure (by ref)") (Volume :type "Float (single-precision)"))
  ;[0 0 0] Enemy Hearing player gunshots
  (if (not (`self.InCombat`))
    (`self.UpdateTargetKey` Instigator)
    (set `self.InCombat` true)
    (`self.AlertNearby` null)
    (bind _asbp_enemy_base (cast `/Game/Blueprints/Enemies/BP_EnemyBase` (`self.Possessed Pawn`)))
    (`/Game/Blueprints/Enemies/BP_EnemyBase.PlayerSpotted` _asbp_enemy_base)))

(event `RemoveAsTarget_Conquest`
  (if (== (`self.PlayerConquest`) (`BlackboardComponent.GetValueAsObject` (`self.Blackboard`) "TargetActor"))
    (`BlackboardComponent.ClearValue` (`self.Blackboard`) "TargetActor")))

(event `RemoveAsTarget_War`
  (if (== (`self.PlayerWar`) (`BlackboardComponent.GetValueAsObject` (`self.Blackboard`) "TargetActor"))
    (`BlackboardComponent.ClearValue` (`self.Blackboard`) "TargetActor")))

(event `RemoveAsTarget_Famine`
  (if (== (`self.PlayerFamine`) (`BlackboardComponent.GetValueAsObject` (`self.Blackboard`) "TargetActor"))
    (`BlackboardComponent.ClearValue` (`self.Blackboard`) "TargetActor")))

(event `RemoveAsTarget_Death`
  (if (== (`self.PlayerDeath`) (`BlackboardComponent.GetValueAsObject` (`self.Blackboard`) "TargetActor"))
    (`BlackboardComponent.ClearValue` (`self.Blackboard`) "TargetActor")))

(fn `Alert`
  (params (TargetActor :type "Actor Object Reference"))
  (`BlackboardComponent.SetValueAsObject` (`self.Blackboard`) "TargetActor" TargetActor))

(fn `UpdateTargetKey`
  (params (Actor :type "Actor Object Reference"))
  (`BlackboardComponent.SetValueAsObject` (`self.Blackboard`) "TargetActor" Actor))

(fn `UserConstructionScript`)