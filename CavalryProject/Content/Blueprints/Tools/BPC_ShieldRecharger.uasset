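; Shield recharger tool that refills a player's shields when it magnetically mounts onto their gear.
; Magnetize picks the nearest free, type-compatible overlapping mount while the tool is neither held nor activated, then disables physics, snaps on and claims the mount.
; Mounting calls Activate, which maxes the shields and notifies the widget handler if the mount's parent is BP_PlayerGear.
; A separate ActivateTool event loops the recharger animation.
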(event `self.Magnetize`
  (params (Magnet :type "Actor Object Reference"))
  (bind _tool_skm (`self.Tool_SkM`))
  (bind _closestmount (`self.ClosestMount`))
  (bind _returnvalue (`SceneComponent.K2_GetComponentLocation` (`self.MagnetCollision`)))
  ;[0 0 0] Magnetic
  (if (`self.toolActivated`)
    _
    (elif (not (`self.IsGrabbed`))
      (set `self.ClosestMount` null)
      (for _array_element (`self.OverlappingMagnets`)
        (if (`/Game/Blueprints/Tools/BP_MagneticPlacement.Occupied` _array_element)
          _
          (elif (or (`|EnumEquality` (`self.Tool Object Type`) (`/Game/Blueprints/Tools/BP_MagneticPlacement.Object Type` _array_element)) (`|EnumEquality` (`/Game/Blueprints/Tools/BP_MagneticPlacement.Object Type` _array_element) "NewEnumerator0"))
            (if (`KismetSystemLibrary.IsValid` (`self.ClosestMount`))
              (if (< (`KismetMathLibrary.VSize` (- _returnvalue (`SceneComponent.K2_GetComponentLocation` (`Actor.RootComponent` _array_element)))) (`KismetMathLibrary.VSize` (- _returnvalue (`SceneComponent.K2_GetComponentLocation` (`Actor.RootComponent` (`self.ClosestMount`))))))
                (set `self.ClosestMount` _array_element))
              (else
                (set `self.ClosestMount` _array_element))))))
      (if (`KismetSystemLibrary.IsValid` (`self.ClosestMount`))
        (`PrimitiveComponent.SetSimulatePhysics` _tool_skm false)
        (`SceneComponent.K2_AttachToComponent` _tool_skm (`Actor.RootComponent` _closestmount) "None" "SnapToTarget" "SnapToTarget" "KeepWorld" false)
        (set `self.OnMagnetMount` true)
        (bind _output_get (set `self.MagnetMount` _closestmount))
        (set `/Game/Blueprints/Tools/BP_MagneticPlacement.Occupied` true _output_get)
        (set `/Game/Blueprints/Tools/BP_MagneticPlacement.AttachedObject` self _output_get)
        (`self.Activate`)))))

(event `/Game/Blueprints/Interfaces/BPI_ToolControls.ActivateTool`
  (params (Active :type Boolean))
  ;[0 0 0] Activates
  (`SkeletalMeshComponent.PlayAnimation` (`self.Tool_SkM`) "/Game/Meshes/Placeholder/Tools/Shield/Shield_Recharger_Out.Shield_Recharger_Out" true))

(event `self.Activate`
  ;[0 0 0] Activates
  (bind _asbp_player_gear (cast `/Game/Blueprints/Characters/Gear/BP_PlayerGear` (`self.GetParentActor` (`self.ClosestMount`))))
  (bind _attachedplayer (`/Game/Blueprints/Characters/Gear/BP_PlayerGear.AttachedPlayer` _asbp_player_gear))
  (set `/Game/Blueprints/Characters/BP_PlayerCharacter_Base.currentShields` (`/Game/Blueprints/Characters/BP_PlayerCharacter_Base.maxShields` _attachedplayer) _attachedplayer)
  ;;[1 1 1] Bean Activate Shields Up
  (`/Game/HUD/Widgets/Damage_Display/BP_HorsemenHUD.BatteryActivated` (`/Game/Blueprints/Characters/BP_PlayerCharacter_Base.WidgetHandler` _attachedplayer)))

(fn `UserConstructionScript`
  (`parent.UserConstructionScript`))