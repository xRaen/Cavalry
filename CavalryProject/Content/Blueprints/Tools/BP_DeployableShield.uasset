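; Throwable, grabbable tool that deploys a shield when it lands.
; Release records the throw location, frees the grab socket and calls Magnetize.
; If the tool is activated, a box collider overlap stops physics and orients it along the throw direction using only X and Y.
; A one-time deploy then spawns and attaches BP_Shield, plays opening animations and sound, and disables grabbing.
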(event `DeployBase`
  (bind _tool_skm (`self.Tool_SkM`))
  ;[0 0 0] Deploy Base and spawn shield
  (`SkeletalMeshComponent.PlayAnimation` _tool_skm "/Game/Meshes/Placeholder/Tools/DeployableShield/OPEN.OPEN" false)
  (bind _returnvalue (`|SpawnActorFromClass` "/Game/Blueprints/Tools/BP_Shield.BP_Shield_C" (`SceneComponent.GetRelativeTransform` _tool_skm) "AlwaysSpawn" "OverrideRootScale" null null))
  (`self.K2_AttachToActor` _returnvalue self "None" "SnapToTarget" "SnapToTarget" "SnapToTarget" false)
  (`SkeletalMeshComponent.PlayAnimation` (`/Game/Blueprints/Tools/BP_Shield.SkM_Shield` _returnvalue) "/Game/Meshes/Placeholder/War/Tool_Shield_Whitebox_01_Opening.Tool_Shield_Whitebox_01_Opening" false)
  (set `/Game/Blueprints/GrabbableObjectSocket.ComponentActive` false (`self.GrabbableObjectSocket`))
  ;;[1 0 1] Shield Spawning Audio
  (`GameplayStatics.PlaySoundAtLocation` "/Game/SFX/Tools/Cavalry_shield_demo_21st_impact.Cavalry_shield_demo_21st_impact" (`SceneComponent.K2_GetComponentLocation` (`self.Tool_SkM`)) (struct) 1.0 1.0 0.0 "/Game/SFX/NewSoundAttenuation.NewSoundAttenuation" null null))

(event `self.Box Collider.OnComponentBeginOverlap`
  (params (OverlappedComponent :type "PrimitiveComponent Object Reference") (OtherActor :type "Actor Object Reference") (OtherComp :type "PrimitiveComponent Object Reference") (OtherBodyIndex :type Integer) (bFromSweep :type Boolean) (SweepResult :type "HitResult Structure (by ref)"))
  (bind (_throwlocation_x _throwlocation_y) (`KismetMathLibrary.BreakVector` (`self.ThrowLocation`)))
  (bind _tool_skm (`self.Tool_SkM`))
  (bind (_returnvalue_x _returnvalue_y) (`KismetMathLibrary.BreakVector` (`SceneComponent.K2_GetComponentLocation` (`self.Tool_SkM`))))
  ;[0 0 0] Landing on Ground
  (`KismetSystemLibrary.PrintString` (`KismetSystemLibrary.GetDisplayName` OtherComp) true true (struct :`R` 1.0 :`G` 0.056108 :`A` 1.0) 20.0)
  (if (`self.toolActivated`)
    (`PrimitiveComponent.SetSimulatePhysics` _tool_skm false)
    (`SceneComponent.K2_SetWorldRotation` _tool_skm (`KismetMathLibrary.FindLookAtRotation` (`KismetMathLibrary.MakeVector` _throwlocation_x _throwlocation_y) (`KismetMathLibrary.MakeVector` _returnvalue_x _returnvalue_y)) false false)
    (`/Engine/EditorBlueprintResources/StandardMacros.DoOnce` false
      (:`Completed`
        (`self.DeployBase`)))))

(event `/Game/Blueprints/Interfaces/BPI_GrabbableObj.Release`
  (params (NewParam :type "EControllerHand Enum" :default "Left"))
  ;[0 0 0] Releasing
  (set `self.ThrowLocation` (`SceneComponent.K2_GetComponentLocation` (`self.Tool_SkM`)))
  (`/Game/Blueprints/GrabbableObjectSocket.Release` (`self.GrabbableObjectSocket`))
  (set `self.isGrabbed` false)
  (`self.Magnetize` null))

(fn `UserConstructionScript`)