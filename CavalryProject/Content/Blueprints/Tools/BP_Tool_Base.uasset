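; Base tool actor that can be grabbed by a hand socket, activated while held, and snapped onto magnetic mounts.
; Grab and Release delegate to GrabbableObjectSocket, and release triggers Magnetize.
; If the tool is inactive, Magnetize attaches it to the nearest overlapping free BP_MagneticPlacement of matching or default type, disabling physics and marking it occupied.
; ActivateTool sets the active state and calls Activate, here only a placeholder print.
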(event `/Game/Blueprints/Interfaces/BPI_GrabbableObj.Grab`
  (params (HandSocket :type Name) (AttachToMe :type "SceneComponent Object Reference") (Actor :type "Actor Object Reference"))
  ;[0 0 0] Grabbing
  (`/Game/Blueprints/GrabbableObjectSocket.Grab` (`self.GrabbableObjectSocket`) (`self.Tool_SkM`) self HandSocket AttachToMe)
  (set `self.isGrabbed` true))

(event `/Game/Blueprints/Interfaces/BPI_GrabbableObj.Release`
  (params (NewParam :type "EControllerHand Enum" :default "Left"))
  ;[0 0 0] Releasing
  (`/Game/Blueprints/GrabbableObjectSocket.Release` (`self.GrabbableObjectSocket`))
  (set `self.isGrabbed` false)
  (`self.Magnetize` null))

(event `Magnetize`
  (params (Magnet :type "Actor Object Reference"))
  (bind _tool_skm (`self.Tool_SkM`))
  (bind _closestmount (`self.ClosestMount`))
  (bind _returnvalue (`SceneComponent.K2_GetComponentLocation` (`self.MagnetCollision`)))
  ;[0 0 0] Magnetic
  (if (`self.toolActivated`)
    _
    (elif (not (`self.IsGrabbed`))
      (set `self.ClosestMount` null)
      (for _array_element (`self.OverlappingMagnets`)
        (if (`/Game/Blueprints/Tools/BP_MagneticPlacement.Occupied` _array_element)
          _
          (elif (or (`|EnumEquality` (`self.Tool Object Type`) (`/Game/Blueprints/Tools/BP_MagneticPlacement.Object Type` _array_element)) (`|EnumEquality` (`/Game/Blueprints/Tools/BP_MagneticPlacement.Object Type` _array_element) "NewEnumerator0"))
            (if (`KismetSystemLibrary.IsValid` (`self.ClosestMount`))
              (if (< (`KismetMathLibrary.VSize` (- _returnvalue (`SceneComponent.K2_GetComponentLocation` (`Actor.RootComponent` _array_element)))) (`KismetMathLibrary.VSize` (- _returnvalue (`SceneComponent.K2_GetComponentLocation` (`Actor.RootComponent` (`self.ClosestMount`))))))
                (set `self.ClosestMount` _array_element))
              (else
                (set `self.ClosestMount` _array_element))))))
      (if (`KismetSystemLibrary.IsValid` (`self.ClosestMount`))
        (`PrimitiveComponent.SetSimulatePhysics` _tool_skm false)
        (`SceneComponent.K2_AttachToComponent` _tool_skm (`Actor.RootComponent` _closestmount) "None" "SnapToTarget" "SnapToTarget" "KeepWorld" false)
        (set `self.OnMagnetMount` true)
        (bind _output_get (set `self.MagnetMount` _closestmount))
        (set `/Game/Blueprints/Tools/BP_MagneticPlacement.Occupied` true _output_get)))))

(event `self.MagnetCollision.OnComponentBeginOverlap`
  (params (OverlappedComponent :type "PrimitiveComponent Object Reference") (OtherActor :type "Actor Object Reference") (OtherComp :type "PrimitiveComponent Object Reference") (OtherBodyIndex :type Integer) (bFromSweep :type Boolean) (SweepResult :type "HitResult Structure (by ref)"))
  ;[0 0 0] Magnetic
  (bind _asbp_magnetic_placement (cast `/Game/Blueprints/Tools/BP_MagneticPlacement` OtherActor))
  (`KismetArrayLibrary.Array_Add` (`self.OverlappingMagnets`) _asbp_magnetic_placement))

(event `self.MagnetCollision.OnComponentEndOverlap`
  (params (OverlappedComponent :type "PrimitiveComponent Object Reference") (OtherActor :type "Actor Object Reference") (OtherComp :type "PrimitiveComponent Object Reference") (OtherBodyIndex :type Integer))
  ;[0 0 0] Magnetic
  (bind _asbp_magnetic_placement (cast `/Game/Blueprints/Tools/BP_MagneticPlacement` OtherActor))
  (`KismetArrayLibrary.Array_RemoveItem` (`self.OverlappingMagnets`) _asbp_magnetic_placement))

(event `/Game/Blueprints/Interfaces/BPI_ToolControls.ActivateTool`
  (params (Active :type Boolean))
  ;[0 0 0] Activates
  (if (`self.isGrabbed`)
    (set `self.toolActivated` Active)
    (`self.Activate`)))

(event `Activate`
  ;[0 0 0] Activates
  (`KismetSystemLibrary.PrintString` "BASE JUNK"))

(fn `UserConstructionScript`)