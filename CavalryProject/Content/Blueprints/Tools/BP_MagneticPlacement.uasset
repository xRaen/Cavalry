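; BP_MagneticPlacement is a magnet point that signals overlapping actors to magnetize to it.
; Both begin and end overlap on CollisionDetection wait briefly, then, if the magnet is not Occupied, send MagnetizeMessage to the other actor with itself and its MagneticLock component.
; The receiving actor handles the response, and this graph only reads Occupied, never sets it.
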(event `self.Collision Detection.OnComponentEndOverlap`
  (params (OverlappedComponent :type "PrimitiveComponent Object Reference") (OtherActor :type "Actor Object Reference") (OtherComp :type "PrimitiveComponent Object Reference") (OtherBodyIndex :type Integer))
  (`KismetSystemLibrary.Delay` 0.1)
  (if (not (`self.Occupied`))
    (message `/Game/Blueprints/Interfaces/BPI_Magnetic.Magnetize` OtherActor self (`self.Magnetic Lock`))))

(event `self.Collision Detection.OnComponentBeginOverlap`
  (params (OverlappedComponent :type "PrimitiveComponent Object Reference") (OtherActor :type "Actor Object Reference") (OtherComp :type "PrimitiveComponent Object Reference") (OtherBodyIndex :type Integer) (bFromSweep :type Boolean) (SweepResult :type "HitResult Structure (by ref)"))
  (`KismetSystemLibrary.Delay` 0.1)
  (if (not (`self.Occupied`))
    (message `/Game/Blueprints/Interfaces/BPI_Magnetic.Magnetize` OtherActor self (`self.Magnetic Lock`))))

(fn `UserConstructionScript`)