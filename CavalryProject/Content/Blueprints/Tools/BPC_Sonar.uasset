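; BPC_Sonar is a grabbable sonar tool that the player switches on and off while holding it.
; Grabbing it off the wall attaches the mesh to a hand socket, records the owning character and starts the tool tutorial.
; Activation interrupts the tutorial and toggles the radar and grid on a 3D_Radar_BP child actor.
; Grab and toggle actions call audio hooks, whose Sonar audio events are empty here.
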(event `Sonar_Activate_Audio`
  ;[1 0 1] Sonar Audio
)

(event `Sonar_Deactivate_Audio`
  ;[1 0 1] Sonar Audio
)

(event `/Game/Blueprints/Interfaces/BPI_ToolControls.ActivateTool`
  (params (Active :type Boolean))
  ;[0 0 0] Activates
  (if (`self.isGrabbed`)
    (`self.InterruptToolTutorial`)
    (if (`self.toolActivated`)
      (set `self.toolActivated` false) ; turn the sonar tool off
      (bind _as3d_radar_bp (cast `/Game/3D_Radar/Blueprints/3D_Radar_BP` (`ChildActorComponent.ChildActor` (`self.3D Radar`))))
      (set `/Game/3D_Radar/Blueprints/3D_Radar_BP.Radar Is Active` false _as3d_radar_bp)
      (set `/Game/3D_Radar/Blueprints/3D_Radar_BP.Grid Is Visible` false _as3d_radar_bp)
      (`self.Sonar_Deactivate_Audio`)
      (else
        (set `self.toolActivated` true) ; Turn the sonar tool on
        (bind _as3d_radar_bp_2 (cast `/Game/3D_Radar/Blueprints/3D_Radar_BP` (`ChildActorComponent.ChildActor` (`self.3D Radar`))))
        (set `/Game/3D_Radar/Blueprints/3D_Radar_BP.Radar Is Active` true _as3d_radar_bp_2)
        (set `/Game/3D_Radar/Blueprints/3D_Radar_BP.Grid Is Visible` true _as3d_radar_bp_2)
        (`self.Sonar_Activate_Audio`)))))

(event `Sonar_Grab_Audio`
  ;[1 0 1] Sonar Audio
)

(event `/Game/Blueprints/Interfaces/BPI_GrabbableObj.Grab`
  (params (HandSocket :type Name) (AttachToMe :type "SceneComponent Object Reference") (Actor :type "Actor Object Reference"))
  ;[0 0 0] Grabbing
  (if (not (`self.OnWall`))
    (`/Game/Blueprints/GrabbableObjectSocket.Grab` (`self.GrabbableObjectSocket`) (`self.Tool_SkM`) self HandSocket AttachToMe)
    (set `self.isGrabbed` true)
    (bind _asbp_player_character_base (cast `/Game/Blueprints/Characters/BP_PlayerCharacter_Base` (`self.GetOwner` Actor)))
    (set `self.ToolOwner` _asbp_player_character_base)
    (`self.ToolTutorial`)
    (`self.Sonar_Grab_Audio`)))

(fn `UserConstructionScript`
  (`parent.UserConstructionScript`))