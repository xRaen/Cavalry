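; BP_SessionSelector is a physical selector in the main menu that hosts or joins an online multiplayer session through overlap triggers.
; Overlapping HandTrigger creates a four-connection, non-LAN session for the first player controller.
; Overlapping HandTrigger1 searches for online sessions and joins the first result, without filtering overlaps or checking that the list has entries.
; Outcomes are reported only through debug strings, and no map travel happens here.
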(event `self.HandTrigger.OnComponentBeginOverlap`
  (params (OverlappedComponent :type "PrimitiveComponent Object Reference") (OtherActor :type "Actor Object Reference") (OtherComp :type "PrimitiveComponent Object Reference") (OtherBodyIndex :type Integer) (bFromSweep :type Boolean) (SweepResult :type "HitResult Structure (by ref)"))
  (`CreateSessionCallbackProxy.CreateSession` (`GameplayStatics.GetPlayerController` 0) 4
    (:`OnSuccess`
      (`KismetSystemLibrary.PrintString` "SESSION CREATED"))
    (:`OnFailure`
      (`KismetSystemLibrary.PrintString` "SESSION CREATION FAILED" true true (struct :`R` 1.0 :`A` 1.0)))))

(event `self.HandTrigger1.OnComponentBeginOverlap`
  (params (OverlappedComponent :type "PrimitiveComponent Object Reference") (OtherActor :type "Actor Object Reference") (OtherComp :type "PrimitiveComponent Object Reference") (OtherBodyIndex :type Integer) (bFromSweep :type Boolean) (SweepResult :type "HitResult Structure (by ref)"))
  (bind _returnvalue (`GameplayStatics.GetPlayerController` 0))
  (bind _results (`FindSessionsCallbackProxy.FindSessions` _returnvalue 5)
    (:`OnSuccess`
      (bind _output (`|GetArrayItem` _results))
      (`KismetSystemLibrary.PrintString` (`KismetStringLibrary.Concat_StrStr` "SESSION FOUND | Server name:  " (`FindSessionsCallbackProxy.GetServerName` _output) " | Current player count: " (`KismetStringLibrary.Conv_IntToString` (`FindSessionsCallbackProxy.GetCurrentPlayers` _output)) " | Max player count: " (`KismetStringLibrary.Conv_IntToString` (`FindSessionsCallbackProxy.GetMaxPlayers` _output)) " | There were " (`KismetStringLibrary.Conv_IntToString` (`KismetArrayLibrary.Array_Length` _results)) " other sessions available"))
      (`JoinSessionCallbackProxy.JoinSession` _returnvalue _output
        (:`OnSuccess`
          (`KismetSystemLibrary.PrintString` "SESSION JOINED"))
        (:`OnFailure`
          (`KismetSystemLibrary.PrintString` "FAILED TO JOIN FOUND SESSION" true true (struct :`R` 1.0 :`A` 1.0)))))
    (:`OnFailure`
      (`KismetSystemLibrary.PrintString` "FAILED TO FIND A SESSION" true true (struct :`R` 1.0 :`A` 1.0)))))

(fn `UserConstructionScript`)