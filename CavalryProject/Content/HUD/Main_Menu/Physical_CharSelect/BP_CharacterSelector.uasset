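; Physical character selection station for the main menu, displaying one horseman from the game instance's character data.
; BeginPlay spawns and attaches the preview character, fills the info and selected-image widgets, and maps every selector by character index.
; Overlapping WidgetTrigger toggles the info widget.
; Overlapping SelectionTrigger sets the player's character through the game instance and player state, shows the selected widget and hides it on other selectors.
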(event `self.ReceiveBeginPlay`
  (bind _asbp_cavalry_game_instance (cast `/Game/HUD/Main_Menu/BP_Cavalry_GameInstance` (`GameplayStatics.GetGameInstance`)))
  (bind _aswidget_cur_horseman_info (cast `/Game/HUD/Main_Menu/Physical_CharSelect/Widget_CurHorsemanInfo` (`WidgetComponent.GetWidget` (`self.CharacterInfo`))))
  (set `self.Horseman_Info` _aswidget_cur_horseman_info)
  (bind (_id _name _description _character _image) (break `/Game/HUD/Main_Menu/Struc_CharacterData` (`|GetArrayItem` (`/Game/HUD/Main_Menu/BP_Cavalry_GameInstance.GetCharacterData` _asbp_cavalry_game_instance) (`self.CurrentCharIndex`))))
  (`/Game/HUD/Main_Menu/Physical_CharSelect/Widget_CurHorsemanInfo.SetCharacterText` _aswidget_cur_horseman_info _name _description)
  (bind _aswidget_selected_char (cast `/Game/HUD/Main_Menu/Physical_CharSelect/Widget_SelectedChar` (`WidgetComponent.GetWidget` (`self.WidgSelectedChar`))))
  (`/Game/HUD/Main_Menu/Physical_CharSelect/Widget_SelectedChar.UpdateImage` _aswidget_selected_char _image)
  (bind _returnvalue (`|SpawnActorFromClass` _character (`KismetMathLibrary.MakeTransform` (0.0 0.0 0.0)) "Undefined" "OverrideRootScale" self null))
  (`self.K2_AttachToComponent` _returnvalue (`self.Horseman_Loc`) "None" "KeepRelative" "KeepRelative" "KeepRelative" true)
  (set `self.CurrentPlayerChar` _returnvalue)
  (bind _outactors (`GameplayStatics.GetAllActorsOfClass` "BP_CharacterSelector_C"))
  (for _array_element _outactors
    (`BlueprintMapLibrary.Map_Add` (`self.Dic_CharSelect`) (`/Game/HUD/Main_Menu/Physical_CharSelect/BP_CharacterSelector.CurrentCharIndex` _array_element) _array_element))
  (if (== (`self.CurrentCharIndex`) (`self.SelectedChar`))
    (`SceneComponent.SetVisibility` (`self.CharacterInfo`) false false)
    (else
      (`SceneComponent.SetVisibility` (`self.WidgSelectedChar`) false false)
      (`SceneComponent.SetVisibility` (`self.CharacterInfo`) false false))))

(event `self.SelectionTrigger.OnComponentBeginOverlap`
  (params (OverlappedComponent :type "PrimitiveComponent Object Reference") (OtherActor :type "Actor Object Reference") (OtherComp :type "PrimitiveComponent Object Reference") (OtherBodyIndex :type Integer) (bFromSweep :type Boolean) (SweepResult :type "HitResult Structure (by ref)"))
  (bind _asbp_player_character_base (cast `/Game/Blueprints/Characters/BP_PlayerCharacter_Base` OtherActor))
  (bind _asbp_cavalry_game_instance (cast `/Game/HUD/Main_Menu/BP_Cavalry_GameInstance` (`GameplayStatics.GetGameInstance`)))
  (bind _asbp_cavalry_playerstate (cast `/Game/HUD/Main_Menu/Multiplayer_Lobby/BP_CavalryPlayerstate` (`Controller.PlayerState` (`Pawn.GetController` _asbp_player_character_base))))
  (`/Game/HUD/Main_Menu/BP_Cavalry_GameInstance.SetCharacter` _asbp_cavalry_game_instance (`self.CurrentCharIndex`) _asbp_cavalry_playerstate)
  (`SceneComponent.SetVisibility` (`self.WidgSelectedChar`) true false)
  (bind _values (`BlueprintMapLibrary.Map_Values` (`self.Dic_CharSelect`)))
  (for _array_element _values
    (set `/Game/HUD/Main_Menu/Physical_CharSelect/BP_CharacterSelector.SelectedChar` (`self.CurrentCharIndex`) _array_element)
    (if (not (== (`/Game/HUD/Main_Menu/Physical_CharSelect/BP_CharacterSelector.CurrentCharIndex` _array_element) (`self.CurrentCharIndex`)))
      (`SceneComponent.SetVisibility` (`/Game/HUD/Main_Menu/Physical_CharSelect/BP_CharacterSelector.WidgSelectedChar` _array_element) false false))))

(event `self.WidgetTrigger.OnComponentBeginOverlap`
  (params (OverlappedComponent :type "PrimitiveComponent Object Reference") (OtherActor :type "Actor Object Reference") (OtherComp :type "PrimitiveComponent Object Reference") (OtherBodyIndex :type Integer) (bFromSweep :type Boolean) (SweepResult :type "HitResult Structure (by ref)"))
  (cast `/Game/Blueprints/Characters/BP_PlayerCharacter_Base` OtherActor)
  (`SceneComponent.SetVisibility` (`self.CharacterInfo`) true false))

(event `self.WidgetTrigger.OnComponentEndOverlap`
  (params (OverlappedComponent :type "PrimitiveComponent Object Reference") (OtherActor :type "Actor Object Reference") (OtherComp :type "PrimitiveComponent Object Reference") (OtherBodyIndex :type Integer))
  (cast `/Game/Blueprints/Characters/BP_PlayerCharacter_Base` OtherActor)
  (`SceneComponent.SetVisibility` (`self.CharacterInfo`) false false))

(fn `UserConstructionScript`)