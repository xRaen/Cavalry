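; Game instance for Cavalry that holds the level list, active level index and menu state, and opens levels by index after a short delay.
; SetGameState spawns world-space menu actors at a fixed transform, reusing valid ones by toggling component visibility, and spawns a loading actor for Loading Screen.
; The Main Menu state shows the MissionBrief actor, while Level Select shows the MainMenu actor.
; VerifyActiveLevelIndex derives the index from the current map name.
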(event `StartNewLevel`
  (params (`Active Level Index` :type Integer))
  (`KismetSystemLibrary.Delay` 0.5)
  (`GameplayStatics.OpenLevel` (`.FileName_18_381C602747293309CC84E4A69220030E` (break `/Game/HUD/Main_Menu/Struc_LevelData` (`|GetArrayItem` (`self.Level Data`) `Active Level Index`))))
  (set `self.Active Level Index` `Active Level Index`))

(fn `Get Level Data`
  (returns (`Level Data` :type "Array of /Game/HUD/Main_Menu/Struc_LevelData Structure"))
  (return (`self.Level Data`)))

(fn `MainMenuVisOff`
  (bind _mainmenu (`self.MainMenu`))
  (`/Engine/EditorBlueprintResources/StandardMacros.IsValid` _mainmenu
    (:`Is Valid`
      (for _array_element (`|MakeArray` (`/Game/HUD/Main_Menu/BP_MainMenu_Actor.MM_Center` _mainmenu) (`/Game/HUD/Main_Menu/BP_MainMenu_Actor.MM_Right` _mainmenu))
        (`SceneComponent.SetVisibility` _array_element false false)
        (return)))
    (:`Is Not Valid`
      (return))))

(fn `MissionBriefVisOff`
  (bind _missionbrief (`self.MissionBrief`))
  (`/Engine/EditorBlueprintResources/StandardMacros.IsValid` _missionbrief
    (:`Is Valid`
      (`SceneComponent.SetVisibility` (`/Game/HUD/Main_Menu/BP_MissionBrief_Actor.StartButton_Widget` _missionbrief) false false))
    (:`Is Not Valid`
      _))
  (return))

(fn `Set Game State`
  (params (NewState :type "/Game/HUD/Main_Menu/EGameState Enum" :default "NewEnumerator1"))
  (returns (`Success?` :type Boolean))
  (bind _missionbrief (`self.MissionBrief`))
  (bind _mainmenu (`self.MainMenu`))
  (if (`|EnumInequality` NewState (`self.Game State`))
    (bind _output_get (set `self.Game State` NewState))
    (switch `/Game/HUD/Main_Menu/EGameState` _output_get
      (:`NewEnumerator1`
        (`/Engine/EditorBlueprintResources/StandardMacros.IsValid` _missionbrief
          (:`Is Valid`
            (`SceneComponent.SetVisibility` (`/Game/HUD/Main_Menu/BP_MissionBrief_Actor.StartButton_Widget` _missionbrief) true false)
            (`self.MainMenuVisOff`))
          (:`Is Not Valid`
            (`self.Spawn MissionBrief`)
            (`self.MainMenuVisOff`)))
        (return true))
      (:`NewEnumerator0`
        (`/Engine/EditorBlueprintResources/StandardMacros.IsValid` _mainmenu
          (:`Is Valid`
            (for _array_element (`|MakeArray` (`/Game/HUD/Main_Menu/BP_MainMenu_Actor.MM_Center` _mainmenu) (`/Game/HUD/Main_Menu/BP_MainMenu_Actor.MM_Right` _mainmenu))
              (`SceneComponent.SetVisibility` _array_element true false)
              (`self.MissionBriefVisOff`)
              (return true)))
          (:`Is Not Valid`
            (`self.Spawn MainMenu`)
            (`self.MissionBriefVisOff`)
            (return true))))
      (:`NewEnumerator2`
        (bind _returnvalue (`|SpawnActorFromClass` "/Game/HUD/Main_Menu/BP_Loading_Actor.BP_Loading_Actor_C" (`KismetMathLibrary.MakeTransform` (-280.0 0.0 100.0)) "Undefined" "OverrideRootScale" null null))
        (set `self.LoadingScreen` _returnvalue)
        (return true)))
    (else
      (return false))))

(fn `Spawn MainMenu`
  (bind _returnvalue (`|SpawnActorFromClass` "/Game/HUD/Main_Menu/BP_MainMenu_Actor.BP_MainMenu_Actor_C" (`KismetMathLibrary.MakeTransform` (-280.0 0.0 100.0)) "Undefined" "OverrideRootScale" null null))
  (set `self.MainMenu` _returnvalue)
  (return))

(fn `Spawn MissionBrief`
  (bind _returnvalue (`|SpawnActorFromClass` "/Game/HUD/Main_Menu/BP_MissionBrief_Actor.BP_MissionBrief_Actor_C" (`KismetMathLibrary.MakeTransform` (-280.0 0.0 100.0)) "Undefined" "OverrideRootScale" null null))
  (set `self.MissionBrief` _returnvalue)
  (return))

(fn `Verify Active Level Index`
  (locals (LocalLevelName :type Name))
  (bind _returnvalue (`GameplayStatics.GetCurrentLevelName` true))
  (bind _output_get (set `local.LocalLevelName` (`KismetStringLibrary.Conv_StringToName` _returnvalue)))
  (if (not (== _output_get (`.FileName_18_381C602747293309CC84E4A69220030E` (break `/Game/HUD/Main_Menu/Struc_LevelData` (`|GetArrayItem` (`self.Level Data`))))))
    (for (_array_element _array_index) (`self.Level Data`) :!label _label
      (if (== (`local.LocalLevelName`) (`.FileName_18_381C602747293309CC84E4A69220030E` (break `/Game/HUD/Main_Menu/Struc_LevelData` _array_element)))
        (set `self.Active Level Index` _array_index)
        (goto _label)))))