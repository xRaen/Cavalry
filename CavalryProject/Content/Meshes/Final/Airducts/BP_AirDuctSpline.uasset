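; Construction-time spline tool that builds an air duct by repeating an instanced mesh along a spline.
; The Construction Script clears the instances, then adds one at each step of mesh length times duct scale along the spline, in local space.
; It sets the spline's Duration to its length, so constant-velocity time lookups act as distance lookups.
; The event graph holds only disabled stubs, so the Blueprint adds no runtime logic.
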(fn `UserConstructionScript`
  (bind _spline (`self.Spline`))
  (set `SplineComponent.Duration` (`SplineComponent.GetSplineLength` _spline) _spline)
  (`InstancedStaticMeshComponent.ClearInstances` (`self.InstancedStaticMesh`))
  (for _index (range (+ (`KismetMathLibrary.FTrunc` (/ (`SplineComponent.GetSplineLength` (`self.Spline`)) (* (`self.MeshLength`) (`self.AirductScale`)))) 1))
    (`InstancedStaticMeshComponent.AddInstance` (`self.InstancedStaticMesh`) (`SplineComponent.GetTransformAtTime` (`self.Spline`) (* _index (* (`self.MeshLength`) (`self.AirductScale`))) "Local" true false))))